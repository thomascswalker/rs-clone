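; Blueprint helper library for the game's UI, giving shared access to the player's main interface, chatbox, inventory and skills windows, plus Shift key state.
; It spawns and clears context menus at the mouse position, interactive hovers labeled with a component's first action and type-styled name, and resource-gathering progress windows.
; Transient widgets are found by class search rather than stored references, and creating a progress window first removes any existing ones.
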(fn IsShiftDown
  (bind _as_player_controller (Utilities|Casting|CastTo_PlayerController (Game|GetPlayerController 0)))
  (return (Variables|/Game/Blueprints/Controllers/_PlayerController._PlayerController_C|GetShiftDown _as_player_controller)))

(fn DestroyContextMenus
  (bind _foundwidgets (Widget|GetAllWidgetsOfClass 0 "/Game/Blueprints/UserInterface/ContextMenu.ContextMenu_C"))
  (for _array_element _foundwidgets
    (Widget|RemovefromParent _array_element)))

(fn CreateContextMenu
  (params (Actors :type Array%20of%20Action%20Structures))
  (bind _returnvalue (Game|GetPlayerController 0))
  (bind (_locationx _locationy) (Game|Player|GetMousePosition _returnvalue))
  (LocalVariables|SetNewLocalVar_1 Actors)
  (bind _returnvalue_2 (UserInterface|CreateWidget "/Game/Blueprints/UserInterface/ContextMenu.ContextMenu_C" (Game|GetPlayerController 0)))
  (bind _output_get (LocalVariables|SetContextMenu _returnvalue_2))
  (UserInterface|Viewport|AddtoViewport _output_get 0)
  (Class|UserWidget|SetPositioninViewport (LocalVariables|GetContextMenu) (Math|Vector2D|MakeVector2D _locationx _locationy) true)
  (Default|OnCreated (LocalVariables|GetContextMenu) (LocalVariables|GetNewLocalVar_1)))

(fn CreateInteractiveHover
  (params (Interactive%20Component :type Interactive%20Component%20Object%20Reference))
  (bind (_action _success) (CallFunction|GetFirstAction Interactive%20Component))
  (if _success
    (bind _returnvalue (UserInterface|CreateWidget "/Game/Blueprints/UserInterface/InteractiveHover.InteractiveHover_C" (Game|GetPlayerController 0)))
    (bind _output_get (LocalVariables|SetWidget _returnvalue))
    (UserInterface|Viewport|AddtoViewport _output_get 0)
    (Rendering|Components|TextRender|SetText (Variables|/Game/Blueprints/UserInterface/InteractiveHover.InteractiveHover_C|GetText (LocalVariables|GetWidget)) (Utilities|Text|ToText(String) (Utilities|String|Append "<Default>" _action "</>" " <" (Utilities|String|EnumtoString (Variables|/Game/Blueprints/Systems/Interaction/InteractiveComponent.InteractiveComponent_C|GetType Interactive%20Component)) ">" (Variables|/Game/Blueprints/Systems/Interaction/InteractiveComponent.InteractiveComponent_C|GetName Interactive%20Component) "</>")))
    (return (LocalVariables|GetWidget))))

(fn DestroyInteractiveHovers
  (bind _foundwidgets (Widget|GetAllWidgetsOfClass 0 "/Game/Blueprints/UserInterface/InteractiveHover.InteractiveHover_C"))
  (for _array_element _foundwidgets
    (Widget|RemovefromParent _array_element)))

(fn GetMainInterface
  (bind _as_player_controller (Utilities|Casting|CastTo_PlayerController (Game|GetPlayerController 0)))
  (return (Variables|/Game/Blueprints/Controllers/_PlayerController._PlayerController_C|GetMainInterface _as_player_controller)))

(fn GetChatbox
  (bind _main_interface (CallFunction|GetMainInterface))
  (bind _chatbox (Variables|/Game/Blueprints/UserInterface/MainInterface.MainInterface_C|GetChatbox _main_interface))
  (Utilities|IsValid _chatbox
    (:Is%20Valid
      (return _chatbox))))

(fn AddChatMessage
  (params (Message :type String) (Color :type ChatboxColors%20Enum :default "NewEnumerator0"))
  (Default|LogMessage (CallFunction|GetChatbox) Message Color))

(fn GetInventory
  (return (Variables|/Game/Blueprints/UserInterface/MainInterface.MainInterface_C|GetInventory (CallFunction|GetMainInterface))))

(fn GetSkills
  (return (Variables|/Game/Blueprints/UserInterface/MainInterface.MainInterface_C|GetSkillsWindow (CallFunction|GetMainInterface))))

(fn CreateProgressWindow
  (params (Steps :type Integer) (Message :type String))
  (CallFunction|DestroyProgressWindows)
  (bind _returnvalue (UserInterface|CreateWidget "/Game/Blueprints/UserInterface/ResourceGatherProgressWindow.ResourceGatherProgressWindow_C" (Game|GetPlayerController 0)))
  (Default|Initialize _returnvalue Steps)
  (UserInterface|Viewport|AddtoViewport _returnvalue 0)
  (Rendering|Components|TextRender|SetText (Variables|/Game/Blueprints/UserInterface/ResourceGatherProgressWindow.ResourceGatherProgressWindow_C|GetMessage _returnvalue) (Utilities|Text|ToText(String) Message)))

(fn DestroyProgressWindows
  (bind _foundwidgets (Widget|GetAllWidgetsOfClass 0 "/Game/Blueprints/UserInterface/ResourceGatherProgressWindow.ResourceGatherProgressWindow_C"))
  (for _array_element _foundwidgets
    (Utilities|IsValid _array_element
      (:Is%20Valid
        (Widget|RemovefromParent _array_element)))))

(fn UpdateProgressWindow
  (params (Progress :type Float%20%28single-precision%29))
  (bind _progresswindow (CallFunction|GetProgressWindow))
  (Utilities|IsValid _progresswindow
    (:Is%20Valid
      (Default|UpdateProgress _progresswindow Progress))))

(fn GetProgressWindow
  (bind _foundwidgets (Widget|GetAllWidgetsOfClass 0 "/Game/Blueprints/UserInterface/ResourceGatherProgressWindow.ResourceGatherProgressWindow_C"))
  (for _array_element _foundwidgets
    (Utilities|IsValid _array_element
      (:Is%20Valid
        (return _array_element)))))