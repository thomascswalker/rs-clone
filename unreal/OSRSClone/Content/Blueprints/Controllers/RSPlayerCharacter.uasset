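; Player character Blueprint with an orbit-and-zoom spring arm camera, which spawns an RSAiController owned by itself on BeginPlay.
; Axis inputs rotate the SpringArm in world space, with pitch clamped to configurable limits and yaw unrestricted.
; The mouse wheel zooms by changing the camera's clamped field of view.
; Task getters expose its TaskComponent, while GetTaskController returns no value.
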(event EventBeginPlay
  (Game|SpawnActorfromClass "/Game/Blueprints/Controllers/RSAiController.RSAiController_C" (Math|Transform|MakeTransform "0, 0, 0" "0, 0, 0" "1,1,1") "Undefined" self 0))

(event Input|AxisEvents|InputAxisUP
  (params (AxisValue :type Float%20%28single-precision%29))
  (bind _limit (Variables|Camera|GetLimit))
  (bind _springarm (Variables|Default|GetSpringArm))
  (bind _returnvalue (Transformation|GetWorldRotation _springarm))
  ;[1 1 1] Camera Rotation
  (Transformation|SetWorldRotation (Variables|Default|GetSpringArm) (Math|Rotator|MakeRotator (.roll _returnvalue) (Math|Float|Clamp(Float) (+ (* AxisValue (Variables|Camera|GetRotationSpeed)) (.pitch _returnvalue)) (.x _limit) (.y _limit)) (.yaw _returnvalue)) false false))

(event Input|AxisEvents|InputAxisRight
  (params (AxisValue :type Float%20%28single-precision%29))
  ;[1 1 1] Camera Rotation
  (Transformation|AddWorldRotation (Variables|Default|GetSpringArm) (Math|Rotator|MakeRotator 0.0 0.0 (* AxisValue (Variables|Camera|GetRotationSpeed))) false false))

(event Input|MouseEvents|MouseWheelAxis
  (params (AxisValue :type Float%20%28single-precision%29))
  ;[1 1 1] Camera zoom
  (Camera|SetFieldOfView (Variables|Default|GetCamera) (Math|Float|Clamp(Float) (- (Variables|/Script/Engine.CameraComponent|GetFieldOfView (Variables|Default|GetCamera)) (* AxisValue (Variables|Camera|GetZoomSpeed))) 2e+01 9e+01)))

(fn ConstructionScript)

(fn GetTaskComponent
  (return (Variables|Default|GetTaskComponent)))

(fn GetTaskController
  (return 0))