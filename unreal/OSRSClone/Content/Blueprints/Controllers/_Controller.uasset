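; Point-and-click player controller that moves the pawn, runs interactions and creates the main UI, with B opening the inventory.
; Cursor traces from the pawn's camera feed left-click movement and right-click context menu creation.
; After a left click, a polling macro waits until the pawn nears the hit, then sends the Interactive's first action.
; Tick tracks the hovered Interactive, firing hover events and clearing custom-depth highlights on all Interactives.
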(event Custom|Left%20Click%20Event
  (bind _targetactor (Variables|Default|GetTargetActor))
  (CallFunction|GetHitsUnderCursor)
  (CallFunction|DestroyAllContextMenus)
  (if (> (Utilities|Array|Length (Variables|Default|GetHits)) 0)
    (CallFunction|GetHitDatafromIndex)
    (CallFunction|MovetoLocation (Variables|Default|GetTargetLocation))
    (Utilities|WaitUntilCloseEnough
      (:Out
        (Utilities|IsValid _targetactor
          (:Is%20Valid
            (bind _asinteractive (Utilities|Casting|CastToInteractive _targetactor))
            (if (.Success (CallFunction|GetFirstAction (Variables|/Game/Blueprints/Systems/Interaction/Interactive.Interactive_C|GetInteractiveComponent _asinteractive)))
              (Class|Interactable|InteractEvent(Message) _asinteractive (.Action (CallFunction|GetFirstAction (Variables|/Game/Blueprints/Systems/Interaction/Interactive.Interactive_C|GetInteractiveComponent _asinteractive))))
              (else
                (Development|PrintString "Object has no actions")))))))))

(event Custom|Right%20Click%20Event
  (CallFunction|GetHitsUnderCursor)
  (CallFunction|CreateContextMenu))

(event EventBeginPlay
  (CallFunction|CreateViewportWidgets)
  (CallFunction|AddChatMessage "Welcome to the game."))

(event EventTick
  (params (DeltaSeconds :type Float%20%28single-precision%29))
  (Utilities|FlowControl|Delay 0.01)
  (bind _out_hits (CallFunction|GetHitsUnderCursor))
  (if (!= (Utilities|Array|Length _out_hits) 0)
    (bind _asinteractive (Utilities|Casting|CastToInteractive (.HitActor (Collision|BreakHitResult (Utilities|Array|Get(acopy) _out_hits))))
      (:then
        (Utilities|IsValid (Variables|Default|GetCurrentFocus)
          (:Is%20Valid
            (if (!= (Variables|Default|GetCurrentFocus) _asinteractive)
              (Default|OnDehover _asinteractive)
              (CallFunction|ClearFocus)
              (bind _output_get (Variables|Default|SetCurrentFocus _asinteractive :!label _label))
              (Default|OnHover _output_get)))
          (:Is%20Not%20Valid
            (goto _label))))
      (:CastFailed
        (Utilities|IsValid (Variables|Default|GetCurrentFocus)
          (:Is%20Valid
            (Default|OnDehover (Variables|Default|GetCurrentFocus)))
          (:Is%20Not%20Valid
            _))
        (Variables|Default|SetCurrentFocus 0)
        (CallFunction|ClearFocus)))))

(event Input|KeyboardEvents|B
  (params (Key :type Key%20Structure :default "None"))
  (bind _main_interface (CallFunction|GetMainInterface))
  (:Pressed
    (Default|OpenTab _main_interface (Variables|/Game/Blueprints/UserInterface/MainInterface.MainInterface_C|GetInventory _main_interface))))

(fn ConstructionScript)

(fn MovetoLocation
  (params (Location :type Vector))
  (LocalVariables|SetGoal Location)
  (if true ; Only move if we're a certain distance away from the target location
    (AI|Navigation|SimpleMovetoLocation self (LocalVariables|GetGoal))
    (return)
    (else
      (return))))

(fn IsInteractive
  (params (Object :type Object%20Object%20Reference))
  (return (Utilities|ClassIsChildOf (Utilities|GetClass Object) "/Game/Blueprints/Systems/Interaction/Interactive.Interactive_C")))

(fn GetHitsUnderCursor
  (bind _as_character (Utilities|Casting|CastTo_Character (Pawn|GetControlledPawn)))
  (Utilities|Array|Add (Variables|Default|GetIgnoreList) _as_character)
  (bind _outhits (Collision|MultiLineTraceByChannel (Transformation|GetWorldLocation (Variables|/Game/Blueprints/Controllers/_Character._Character_C|GetCamera _as_character)) (+ (Transformation|GetWorldLocation (Variables|/Game/Blueprints/Controllers/_Character._Character_C|GetCamera _as_character)) (* (.WorldDirection (Game|Player|ConvertMouseLocationToWorldSpace)) (Variables|Default|GetTraceDistance))) "TraceTypeQuery1" false (Variables|Default|GetIgnoreList) "None" true "(R=1.000000,G=0.000000,B=0.000000,A=1.000000)" "(R=0.000000,G=1.000000,B=0.000000,A=1.000000)" 1.0))
  (Variables|Default|SetHits _outhits)
  (return _outhits))

(fn GetCloseEnough
  (params (Component :type Primitive%20Component%20Object%20Reference))
  (bind _returnvalue (Pawn|GetControlledPawn))
  (bind _returnvalue_2 (Transformation|GetActorLocation _returnvalue))
  (bind (_x _y) (Math|Vector|BreakVector _returnvalue_2))
  (bind _outpointonbody (Collision|GetClosestPointonCollision Component _returnvalue_2 "None"))
  (return (< (Math|Vector|Distance(Vector) (Math|Vector|MakeVector (.x _outpointonbody) (.y _outpointonbody) 0.0) (Math|Vector|MakeVector _x _y 0.0)) (Variables|Default|GetMovementThreshold))))

(fn GetHitDatafromIndex
  (params (Index :type Integer))
  (bind _hits (Variables|Default|GetHits))
  (bind _output (Utilities|Array|Get(acopy) _hits Index))
  (bind (_bblockinghit _binitialoverlap _time _distance _location _impactpoint _normal _impactnormal _physmat _hitactor _hitcomponent) (Collision|BreakHitResult _output))
  (Utilities|IsValid _hitactor
    (:Is%20Valid
      (Variables|Default|SetTargetLocation _location)
      (Variables|Default|SetHitPoint _impactpoint)
      (Variables|Default|SetTargetActor _hitactor)
      (Variables|Default|SetHit%20Component _hitcomponent)
      (return))))

(fn DestroyAllContextMenus
  (bind _foundwidgets (Widget|GetAllWidgetsOfClass "/Game/Blueprints/UserInterface/ContextMenu.ContextMenu_C" true))
  (for _array_element _foundwidgets
    (Widget|SetVisibility _array_element "Hidden")))

(fn CreateViewportWidgets
  (bind _returnvalue (UserInterface|CreateWidget "/Game/Blueprints/UserInterface/MainInterface.MainInterface_C" (Game|GetPlayerController 0)))
  (bind _output_get (Variables|Default|SetMainInterface _returnvalue))
  (UserInterface|Viewport|AddtoViewport _output_get 0))

(fn PickupItem
  (Development|PrintString "Hello"))

(fn CreateContextMenu
  (bind _returnvalue (Game|GetPlayerController 0))
  (bind (_locationx _locationy) (Game|Player|GetMousePosition _returnvalue))
  (bind _returnvalue_2 (UserInterface|CreateWidget "/Game/Blueprints/UserInterface/ContextMenu.ContextMenu_C" (Game|GetPlayerController 0)))
  (bind _output_get (LocalVariables|SetContextMenu _returnvalue_2))
  (UserInterface|Viewport|AddtoViewport _output_get 0)
  (Class|UserWidget|SetPositioninViewport (LocalVariables|GetContextMenu) (Math|Vector2D|MakeVector2D _locationx _locationy) true))

(fn GetHitActions
  (for _array_element (Variables|Default|GetHits)
    (bind _asinteractive (Utilities|Casting|CastToInteractive (.hitactor _array_element)))
    (Utilities|Array|Add :TargetArray (LocalVariables|GetTempActions))))

(fn PickupItem0
  (Development|PrintString "Hello"))

(fn ClearFocus
  (Utilities|FlowControl|Sequence
    (:then_0
      (Variables|Default|SetCurrentFocus 0))
    (:then_1
      (bind _outactors (Actor|GetAllActorsOfClass "/Game/Blueprints/Systems/Interaction/Interactive.Interactive_C"))
      (for _array_element _outactors
        (Rendering|SetRenderCustomDepth (Variables|/Game/Blueprints/Systems/Interaction/Interactive.Interactive_C|GetStaticMesh _array_element) false)))))

(fn Moveto
  (params (Location :type Vector :default "0, 0, 0"))
  (return false))