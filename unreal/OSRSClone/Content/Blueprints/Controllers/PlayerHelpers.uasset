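; PlayerHelpers is a set of helper functions for reaching a player's inventory and skills and for computing level experience.
; GetController casts the indexed player controller to the custom _PlayerController, which supplies the Inventory and Skills getters.
; Skill level, icon and experience lookups linearly search player 0's skills by type.
; GetLevelExperience sums a truncated exponential term per level, a RuneScape-style curve that doubles roughly every seven levels.
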(fn GetController
  (params (Player :type Integer))
  (bind _as_player_controller (Utilities|Casting|CastTo_PlayerController (Game|GetPlayerController 0 Player)))
  (return _as_player_controller))

(fn GetInventory
  (params (Player :type Integer))
  (return (Variables|/Game/Blueprints/Controllers/_PlayerController._PlayerController_C|GetInventory (CallFunction|GetController Player))))

(fn GetSkills
  (params (Player :type Integer))
  (return (Variables|/Game/Blueprints/Controllers/_PlayerController._PlayerController_C|GetSkills (CallFunction|GetController Player))))

(fn GetSkillLevel
  (params (Type :type Skills%20Enum :default "NewEnumerator0"))
  (for _array_element (Variables|/Game/Blueprints/Systems/Skills/SkillComponent.SkillComponent_C|GetSkills (CallFunction|GetSkills))
    (if (Utilities|Enum|Equal(Enum) Type (.name _array_element))
      (return (.level _array_element)))))

(fn GetSkillIcon
  (params (Type :type Skills%20Enum :default "NewEnumerator0"))
  (for _array_element (Variables|/Game/Blueprints/Systems/Skills/SkillComponent.SkillComponent_C|GetSkills (CallFunction|GetSkills))
    (if (Utilities|Enum|Equal(Enum) Type (.name _array_element))
      (return (.icon _array_element)))))

(fn GetSkillExperience
  (params (Type :type Skills%20Enum :default "NewEnumerator0"))
  (for _array_element (Variables|/Game/Blueprints/Systems/Skills/SkillComponent.SkillComponent_C|GetSkills (CallFunction|GetSkills))
    (if (Utilities|Enum|Equal(Enum) Type (.name _array_element))
      (return (.experience _array_element)))))

(fn GetLevelExperience
  (params (Level :type Integer) (__WorldContext :type Object%20Object%20Reference))
  (for _index (range 1 Level)
    (bind _output_get (LocalVariables|SetFloatLevel (Math|Conversions|ToFloat(Integer) _index)))
    (LocalVariables|SetTotalExperience (+ (LocalVariables|GetTotalExperience) (Math|Float|Truncate (/ (+ (- _output_get 1.0) (* (Math|Float|Power 2.0 (/ (- (LocalVariables|GetFloatLevel) 1.0) 7.0)) 3e+02)) 4.0)))))
  (return (LocalVariables|GetTotalExperience)))