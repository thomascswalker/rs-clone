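; Base character Blueprint that handles player camera orbit and zoom around a spring arm.
; The vertical input axis pitches the arm in local space and the horizontal axis yaws it in world space, both scaled by a rotation speed.
; Mouse wheel input changes the arm length by a zoom speed, clamped to a fixed range.
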(event EventBeginPlay)

(event Input|AxisEvents|InputAxisUP
  (params (AxisValue :type Float%20%28single-precision%29))
  ;[1 1 1] Camera Rotation
  (Transformation|AddLocalRotation (Variables|Default|GetSpringArm) (Math|Rotator|MakeRotator 0.0 (* AxisValue (Variables|Camera|GetRotationSpeed)) 0.0) false false))

(event Input|AxisEvents|InputAxisRight
  (params (AxisValue :type Float%20%28single-precision%29))
  ;[1 1 1] Camera Rotation
  (Transformation|AddWorldRotation (Variables|Default|GetSpringArm) (Math|Rotator|MakeRotator 0.0 0.0 (* AxisValue (Variables|Camera|GetRotationSpeed))) false false))

(event Input|MouseEvents|MouseWheelAxis
  (params (AxisValue :type Float%20%28single-precision%29))
  (bind _springarm (Variables|Default|GetSpringArm))
  ;[1 1 1] Camera zoom
  (Variables|/Script/Engine.SpringArmComponent|SetTargetArmLength _springarm (Math|Float|Clamp(Float) (- (Variables|/Script/Engine.SpringArmComponent|GetTargetArmLength _springarm) (* AxisValue (Variables|Camera|GetZoomSpeed))) 2.5e+02 1.2e+03)))

(fn ConstructionScript)