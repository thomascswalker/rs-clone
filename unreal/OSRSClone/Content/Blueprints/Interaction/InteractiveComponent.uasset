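; Actor component that gives its owning actor click and hover state for mouse interaction.
; On BeginPlay it binds to the owner's click and cursor-over events and caches the owner's valid static mesh components.
; Clicks toggle the clicked state and the cursor sets the hover state, each then calling SetHighlight.
; SetHighlight only tests those flags and applies no visual change; the cached meshes are not yet used.
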(event Custom|OnClicked
  (params (TouchedActor :type Actor%20Object%20Reference) (ButtonPressed :type Key%20Structure))
  (Variables|Default|SetIsClicked (not (Variables|Default|GetIsClicked)))
  (CallFunction|SetHighlight))

(event Custom|OnHovered
  (params (TouchedActor :type Actor%20Object%20Reference))
  (Variables|Default|SetIsHovered true)
  (CallFunction|SetHighlight))

(event Custom|OnDehovered
  (params (TouchedActor :type Actor%20Object%20Reference))
  (Variables|Default|SetIsHovered false)
  (CallFunction|SetHighlight))

(event EventBeginPlay
  (bind _returnvalue (Components|GetOwner))
  (EventDispatchers|BindEventtoOnClicked _returnvalue (delegate Custom|OnClicked))
  (EventDispatchers|BindEventtoOnBeginCursorOver _returnvalue (delegate Custom|OnHovered))
  (EventDispatchers|BindEventtoOnEndCursorOver _returnvalue (delegate Custom|OnDehovered))
  (CallFunction|BuildMeshRef))

(fn SetHighlight
  (if (or (Variables|Default|GetIsClicked) (Variables|Default|GetIsHovered))
    _))

(fn BuildMeshRef
  (for _array_element (Actor|GetComponentsByClass (Components|GetOwner) "/Script/Engine.StaticMeshComponent")
    (Utilities|IsValid _array_element
      (:Is%20Valid
        (Utilities|Array|Add (Variables|Default|GetStaticMeshRef) _array_element)))))