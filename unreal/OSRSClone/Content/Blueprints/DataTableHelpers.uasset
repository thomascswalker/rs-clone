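; Helper functions that look up rows in the ItemData data table by item name or by row position.
; GetItemIndexFromName scans every row for a matching Name field, returning its index and row name, or -1 and None when absent.
; GetItemFromName resolves that index and passes it to GetItemFromIndex, which walks the row names to that position and returns the row's data.
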(fn GetItemIndexfromName
  (params (Name :type String))
  (bind _outrownames (DataTable|GetDataTableRowNames "/Game/Blueprints/Systems/Interaction/ItemData.ItemData"))
  (for (_array_element _array_index) _outrownames
    (bind _returnvalue (Utilities|GetDataTableRow "/Game/Blueprints/Systems/Interaction/ItemData.ItemData" _array_element)
      (:then
        (if (Utilities|Enum|Equal(Enum) (.name _returnvalue) Name)
          (return _array_index _array_element)))))
  (return -1 "None"))

(fn GetItemfromName
  (params (Name :type String))
  (bind _index (CallFunction|GetItemIndexfromName Name))
  (if (> _index -1)
    (return (CallFunction|GetItemfromIndex _index))))

(fn GetItemfromIndex
  (params (Index :type Integer))
  (bind _outrownames (DataTable|GetDataTableRowNames "/Game/Blueprints/Systems/Interaction/ItemData.ItemData"))
  (for (_array_element _array_index) _outrownames
    (if (== _array_index Index)
      (bind _returnvalue (Utilities|GetDataTableRow "/Game/Blueprints/Systems/Interaction/ItemData.ItemData" _array_element)
        (:then
          (return _returnvalue))))))