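; Base world item actor that can be examined or picked up into the player's inventory.
; Its construction script reads a data table row into ItemComponent properties, then applies the mesh, name and examine text.
; Pickup interaction sends itself and its quantity to the controller's inventory widget, while the PickedUp event destroys it and notifies any valid spawner.
; A helper converts one-based indices to row names.
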(event EventExamineEvent
  (Development|PrintString (Variables|/Game/Blueprints/Interaction/InteractiveComponent.InteractiveComponent_C|GetExamineText (Variables|Default|GetInteractiveComponent))))

(event EventPickedUp
  (bind _spawner (Variables|Default|GetSpawner))
  (Actor|DestroyActor)
  (Utilities|IsValid _spawner
    (:Is%20Valid
      (Default|OnPickedUp _spawner))))

(event EventInteractEvent
  (params (Action :type String))
  (switch string Action
    (:Pickup
      (bind _as_controller (Utilities|Casting|CastTo_Controller (Game|GetPlayerController 0)))
      (Default|Add (Variables|/Game/Blueprints/Controllers/_Controller._Controller_C|GetInventoryWidget _as_controller) self (Variables|/Game/Blueprints/Items/ItemComponent.ItemComponent_C|GetProperties (Variables|Default|GetItemComponent)) (Variables|Default|GetQuantity)))))

(fn ConstructionScript
  (bind _interactivecomponent (Variables|Default|GetInteractiveComponent))
  (bind _returnvalue (Utilities|GetDataTableRow "/Game/Blueprints/Items/ItemData.ItemData" (.rowname (Variables|Default|GetRow)))
    (:then
      (bind _output_get (Variables|/Game/Blueprints/Items/ItemComponent.ItemComponent_C|SetProperties (Variables|Default|GetItemComponent) (Utilities|Struct|MakeItemProperties (.name _returnvalue) (.mesh _returnvalue) (.icon _returnvalue) (.stackable _returnvalue) 1 0 (.description _returnvalue) 0)))
      (Utilities|FlowControl|Sequence
        (:then_0
          (Components|StaticMesh|SetStaticMesh (Variables|Default|GetStaticMesh) (.mesh _output_get)))
        (:then_1
          (Variables|/Game/Blueprints/Interaction/InteractiveComponent.InteractiveComponent_C|SetName _interactivecomponent (.name _output_get)))
        (:then_2
          (Variables|/Game/Blueprints/Interaction/InteractiveComponent.InteractiveComponent_C|SetExamineText _interactivecomponent (.description _output_get)))))))

(fn GetDataTableNamefromIndex
  (params (Index :type Integer))
  (bind _outrownames (DataTable|GetDataTableRowNames "/Game/Blueprints/Items/ItemData.ItemData"))
  (for (_array_element _array_index) _outrownames
    (if (== (+ _array_index 1) Index)
      (return _array_element))))