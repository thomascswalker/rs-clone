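; Item spawner actor that places a data-table-defined item at its location and respawns it after pickup.
; On BeginPlay it spawns the item at its root transform, passing the row, quantity and itself as spawner.
; When OnPickedUp fires and the item is no longer valid, it waits SpawnTime before spawning again.
; The construction script previews the row's icon on a billboard, plus quantity text for stackable items.
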(event Custom|OnPickedUp
  (Utilities|IsValid (Variables|Item|GetItem)
    (:Is%20Not%20Valid
      (Utilities|FlowControl|Delay (Variables|Properties|GetSpawnTime))
      (CallFunction|Spawn))))

(event EventBeginPlay
  (CallFunction|Spawn))

(fn ConstructionScript
  (bind _textrender (Variables|Default|GetTextRender))
  (bind _returnvalue (Utilities|GetDataTableRow "/Game/Blueprints/Items/ItemData.ItemData" (.rowname (Variables|Item|GetRow)))
    (:then
      (if (.stackable _returnvalue)
        (Rendering|SetVisibility _textrender true false)
        (Rendering|Components|TextRender|SetText _textrender (Utilities|Text|ToText(Integer) (Variables|Item|GetQuantity))))
      (Rendering|Components|Sprite|SetSprite (Variables|Default|GetBillboard) (.icon _returnvalue)))))

(fn Spawn
  (bind _returnvalue (Game|SpawnActorfromClass "/Game/Blueprints/Items/Item.Item_C" (Transformation|GetWorldTransform (Variables|Default|GetDefaultSceneRoot)) "Undefined" 0 0 (Variables|Item|GetRow) 1 0))
  (Variables|Item|SetItem _returnvalue)
  (Variables|/Game/Blueprints/Items/Item.Item_C|SetQuantity _returnvalue (Variables|Item|GetQuantity))
  (Variables|/Game/Blueprints/Items/Item.Item_C|SetSpawner _returnvalue self))