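; PathGrid is a tile grid actor that previews an A* path from the selected tile to the hovered tile.
; CreateMapData spawns PathTile actors, classifies walkability with two sphere-trace channels and maps them by coordinate, at BeginPlay or during construction when ShowGrid is on.
; Hovering runs FindPathToTarget over eight-way walkable neighbors using Manhattan distance for cost and heuristic, then RetracePath follows PreviousTile links to flag and store the path.
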(event Custom|OnTileSelected
  (params (Tile :type Path%20Tile%20Object%20Reference))
  (Utilities|IsValid (Variables|Path|GetSelectedTile)
    (:Is%20Valid
      (Default|DeselectTile (Variables|Path|GetSelectedTile)))
    (:Is%20Not%20Valid
      _))
  (Variables|Path|SetSelectedTile Tile))

(event Custom|OnTileHovered
  (params (Tile :type Path%20Tile%20Object%20Reference))
  (Utilities|IsValid (Variables|Path|GetHoveredTile)
    (:Is%20Valid
      (Default|DehoverTile (Variables|Path|GetHoveredTile)))
    (:Is%20Not%20Valid
      _))
  (Variables|Path|SetHoveredTile Tile)
  (CallFunction|ClearPath)
  (if (and (Utilities|IsValid (Variables|Path|GetSelectedTile)) (Utilities|IsValid (Variables|Path|GetHoveredTile)))
    (CallFunction|FindPathtoTarget (Variables|Path|GetSelectedTile) (Variables|Path|GetHoveredTile))))

(event EventBeginPlay
  (CallFunction|CreateMapData))

(fn ConstructionScript
  (bind _gridsizeworld (Variables|Grid|GetGridSizeWorld))
  (Rendering|Debug|FlushPersistentDebugLines)
  (if (Variables|Debug|GetShowGrid)
    (CallFunction|CreateMapData)
    (Rendering|Debug|DrawDebugBox "0, 0, 0" (Math|Vector|MakeVector (.x _gridsizeworld) (.y _gridsizeworld) 5.0) (Variables|Debug|GetGridBoundsColor) "0, 0, 0" 9999999.0 1e+01)))

(fn ClearPath
  (bind _values (Utilities|Map|Values (Variables|Grid|GetTileData)))
  (for _array_element _values
    (Default|SetColor _array_element)))

(fn CreateMapData
  (bind (_gridtilex _gridtiley) (CallFunction|GetTileCount))
  (Variables|Grid|SetGridLocation (Transformation|GetWorldLocation (Variables|Default|GetScene)))
  (for _index (range 0 _gridtilex)
    (LocalVariables|SetX _index)
    (for _index_2 (range 0 _gridtiley)
      (LocalVariables|SetY _index_2)
      (bind _output_get (LocalVariables|SetTilePosition (CallFunction|GetTilePositionfromCoordinate (LocalVariables|GetX) (LocalVariables|GetY))))
      (LocalVariables|SetWalkable (and (CallFunction|TraceTile _output_get "TraceTypeQuery3") (not (CallFunction|TraceTile _output_get "TraceTypeQuery4"))))
      (Utilities|FlowControl|Sequence
        (:then_0
          (if (LocalVariables|GetWalkable)
            (LocalVariables|SetType "NewEnumerator1")
            (else
              (LocalVariables|SetType "NewEnumerator2"))))
        (:then_1
          (bind _returnvalue (Game|SpawnActorfromClass "/Game/Blueprints/Pathfinding/PathTile.PathTile_C" (Math|Conversions|ToTransform(Vector) (LocalVariables|GetTilePosition)) "Undefined" 0 0))
          (LocalVariables|SetTile _returnvalue)
          (Variables|/Game/Blueprints/Pathfinding/PathTile.PathTile_C|SetType (LocalVariables|GetTile) (LocalVariables|GetType))
          (Variables|/Game/Blueprints/Pathfinding/PathTile.PathTile_C|SetIndex (LocalVariables|GetTile) (Math|Vector2D|MakeVector2D (Math|Conversions|ToFloat(Integer) (LocalVariables|GetX)) (Math|Conversions|ToFloat(Integer) (LocalVariables|GetY))))
          (Variables|/Game/Blueprints/Pathfinding/PathTile.PathTile_C|SetGrid (LocalVariables|GetTile) self))
        (:then_2
          (Utilities|Map|Add (Variables|Grid|GetTileData) (Math|Vector2D|MakeVector2D (Math|Conversions|ToFloat(Integer) (LocalVariables|GetX)) (Math|Conversions|ToFloat(Integer) (LocalVariables|GetY))) (LocalVariables|GetTile)))))))

(fn FindPathtoTarget
  (params (Start :type Path%20Tile%20Object%20Reference) (Target :type Path%20Tile%20Object%20Reference))
  (CallFunction|ClearPath)
  ;[1 1 1] Initial variables
  (LocalVariables|SetStartIndex Start)
  (LocalVariables|SetTargetIndex Target)
  (LocalVariables|SetCurrentIndex (LocalVariables|GetStartIndex))
  (Utilities|Array|AddUnique (LocalVariables|GetOpenSet) (LocalVariables|GetStartIndex))
  ;[1 1 1] Main loop
  (while (> (Utilities|Array|Length (LocalVariables|GetOpenSet)) 0)
    (LocalVariables|SetCurrentIndex (Utilities|Array|Get(acopy) (LocalVariables|GetOpenSet)))
    (for _array_element (LocalVariables|GetOpenSet)
      ;[1 1 1] See if there's a cheaper tile to go to
      (if (and (or (< (Default|GetFCost _array_element) (Default|GetFCost (LocalVariables|GetCurrentIndex))) (== (Default|GetFCost _array_element) (Default|GetFCost (LocalVariables|GetCurrentIndex)))) (< (Variables|/Game/Blueprints/Pathfinding/PathTile.PathTile_C|GetHCost _array_element) (Variables|/Game/Blueprints/Pathfinding/PathTile.PathTile_C|GetHCost (LocalVariables|GetCurrentIndex))))
        (LocalVariables|SetCurrentIndex _array_element)))
    (Utilities|Array|RemoveItem (LocalVariables|GetOpenSet) (LocalVariables|GetCurrentIndex))
    (Utilities|Array|AddUnique (LocalVariables|GetClosedSet) (LocalVariables|GetCurrentIndex))
    (if (Math|Vector|Equal(Vector) (Variables|/Game/Blueprints/Pathfinding/PathTile.PathTile_C|GetIndex (LocalVariables|GetCurrentIndex)) (Variables|/Game/Blueprints/Pathfinding/PathTile.PathTile_C|GetIndex (LocalVariables|GetTargetIndex)) 0.0001)
      ;[1 1 1] Retrace
      (CallFunction|RetracePath (LocalVariables|GetTargetIndex) (LocalVariables|GetStartIndex))
      (return)
      (else
        ;[1 1 1] For each neighboring tile
        (for _array_element_2 (CallFunction|GetNeighbors (LocalVariables|GetCurrentIndex))
          ;[1 1 1] Continue the loop if the closed set already contains the neighbor
          (bind _output_get (LocalVariables|SetNeighbor _array_element_2))
          (if (not (Utilities|Array|ContainsItem (LocalVariables|GetClosedSet) _output_get))
            (if (or (not (Utilities|Array|ContainsItem (LocalVariables|GetOpenSet) (LocalVariables|GetNeighbor))) (< (+ (Variables|/Game/Blueprints/Pathfinding/PathTile.PathTile_C|GetGCost (LocalVariables|GetCurrentIndex)) (CallFunction|GetDistance (LocalVariables|GetCurrentIndex) (LocalVariables|GetNeighbor))) (Variables|/Game/Blueprints/Pathfinding/PathTile.PathTile_C|GetGCost (LocalVariables|GetNeighbor))))
              (Variables|/Game/Blueprints/Pathfinding/PathTile.PathTile_C|SetGCost (LocalVariables|GetNeighbor) (+ (Variables|/Game/Blueprints/Pathfinding/PathTile.PathTile_C|GetGCost (LocalVariables|GetCurrentIndex)) (CallFunction|GetDistance (LocalVariables|GetCurrentIndex) (LocalVariables|GetNeighbor))))
              (Variables|/Game/Blueprints/Pathfinding/PathTile.PathTile_C|SetHCost (LocalVariables|GetNeighbor) (CallFunction|GetDistance (LocalVariables|GetNeighbor) (LocalVariables|GetTargetIndex)))
              (Variables|/Game/Blueprints/Pathfinding/PathTile.PathTile_C|SetPreviousTile (LocalVariables|GetNeighbor) (LocalVariables|GetCurrentIndex))
              (if (not (Utilities|Array|ContainsItem (LocalVariables|GetOpenSet) (LocalVariables|GetNeighbor)))
                (Utilities|Array|AddUnique (LocalVariables|GetOpenSet) (LocalVariables|GetNeighbor))))))))))

(fn GetDistance
  (params (From :type Path%20Tile%20Object%20Reference) (To :type Path%20Tile%20Object%20Reference))
  ;[1 1 1] Get whether we move in X, or move in Y
  (LocalVariables|SetTileA From)
  (LocalVariables|SetTileB To)
  (return (+ (Math|Float|Round (Math|Float|Absolute(Float) (.x (- (Variables|/Game/Blueprints/Pathfinding/PathTile.PathTile_C|GetIndex (LocalVariables|GetTileA)) (Variables|/Game/Blueprints/Pathfinding/PathTile.PathTile_C|GetIndex (LocalVariables|GetTileB)))))) (Math|Float|Round (Math|Float|Absolute(Float) (.y (- (Variables|/Game/Blueprints/Pathfinding/PathTile.PathTile_C|GetIndex (LocalVariables|GetTileA)) (Variables|/Game/Blueprints/Pathfinding/PathTile.PathTile_C|GetIndex (LocalVariables|GetTileB)))))))))

(fn GetNeighbors
  (params (Tile :type Path%20Tile%20Object%20Reference))
  (Utilities|FlowControl|Sequence
    (:then_0
      ;[1 1 1] Get possible neighbor indexes
      (for _index (range -1 1)
        (for _index_2 (range -1 1)
          (if (Math|Vector|NotEqual(Vector) :A (Math|Vector2D|MakeVector2D (Math|Conversions|ToFloat(Integer) _index) (Math|Conversions|ToFloat(Integer) _index_2)))
            (Utilities|Array|Add (LocalVariables|GetPossible) (Math|Vector2D|MakeVector2D (Math|Conversions|ToFloat(Integer) _index) (Math|Conversions|ToFloat(Integer) _index_2)))))))
    (:then_1
      (for _array_element (LocalVariables|GetPossible)
        (Utilities|IsValid (.Value (Utilities|Map|Find (Variables|Grid|GetTileData) (+ _array_element (Variables|/Game/Blueprints/Pathfinding/PathTile.PathTile_C|GetIndex Tile))))
          (:Is%20Valid
            (if (and (Utilities|Enum|Equal(Enum) (Variables|/Game/Blueprints/Pathfinding/PathTile.PathTile_C|GetType (.Value (Utilities|Map|Find (Variables|Grid|GetTileData) (+ _array_element (Variables|/Game/Blueprints/Pathfinding/PathTile.PathTile_C|GetIndex Tile))))) "NewEnumerator1") (.ReturnValue (Utilities|Map|Find (Variables|Grid|GetTileData) (+ _array_element (Variables|/Game/Blueprints/Pathfinding/PathTile.PathTile_C|GetIndex Tile)))))
              (Utilities|Array|AddUnique (LocalVariables|GetValidNeighbors) (.Value (Utilities|Map|Find (Variables|Grid|GetTileData) (+ _array_element (Variables|/Game/Blueprints/Pathfinding/PathTile.PathTile_C|GetIndex Tile)))))))))
      (return (LocalVariables|GetValidNeighbors)))))

(fn GetOrigin
  (return (- (- (Variables|Grid|GetGridLocation) (* (Math|Vector|GetRightVector (Variables|Default|GetScene)) (.x (Variables|Grid|GetGridSizeWorld)))) (* (Math|Vector|GetForwardVector (Variables|Default|GetScene)) (.y (Variables|Grid|GetGridSizeWorld))))))

(fn GetRealTileSize
  (return (- (Variables|Grid|GetTileSize) (Variables|Grid|GetTileGap))))

(fn GetTileCount
  (bind _tilesize (Variables|Grid|GetTileSize))
  (bind _tilecount (Variables|Grid|GetTileCount))
  (bind _tilecount_2 (Variables|Grid|GetTileCount))
  (bind _returnvalue (* _tilecount _tilesize))
  (Variables|Grid|SetGridSizeWorld (Math|Vector2D|MakeVector2D _returnvalue _returnvalue))
  (return _tilecount_2 _tilecount_2))

(fn GetTilefromIndex
  (params (Index :type Vector%202D%20Structure%20%28by%20ref%29))
  (return (.Value (Utilities|Map|Find (Variables|Grid|GetTileData) Index))))

(fn GetTilefromPosition
  (params (Position :type Vector))
  (bind _gridsizeworld (Variables|Grid|GetGridSizeWorld))
  (bind _gridsizeworld_2 (Variables|Grid|GetGridSizeWorld))
  (bind _tilecount (Variables|Grid|GetTileCount))
  (bind _returnvalue (- _tilecount 1))
  (bind _returnvalue_2 (/ _gridsizeworld 2.0))
  (bind _returnvalue_3 (+ (.y Position) (.y _returnvalue_2)))
  (bind _returnvalue_4 (+ (.x Position) (.x _returnvalue_2)))
  (bind _returnvalue_5 (/ _returnvalue_3 (.y _gridsizeworld_2)))
  (bind _returnvalue_6 (/ _returnvalue_4 (.x _gridsizeworld_2)))
  (bind _returnvalue_7 (Math|Float|Clamp(Float) _returnvalue_5))
  (bind _returnvalue_8 (Math|Float|Clamp(Float) _returnvalue_6))
  (bind _returnvalue_9 (* _returnvalue _returnvalue_7))
  (bind _returnvalue_10 (* _returnvalue _returnvalue_8))
  (bind _returnvalue_11 (Math|Float|Truncate _returnvalue_9))
  (bind _returnvalue_12 (Math|Float|Truncate _returnvalue_10))
  (bind _returnvalue_13 (Math|Conversions|ToFloat(Integer) _returnvalue_12))
  (bind _returnvalue_14 (Math|Conversions|ToFloat(Integer) _returnvalue_11))
  (bind _returnvalue_15 (Math|Vector2D|MakeVector2D _returnvalue_13 _returnvalue_14))
  (bind _tile (CallFunction|GetTilefromIndex _returnvalue_15))
  (Utilities|IsValid _tile
    (:Is%20Valid
      (return _tile))))

(fn GetTilePositionfromCoordinate
  (params (X :type Integer) (Y :type Integer))
  (bind _tilesize (Variables|Grid|GetTileSize))
  (bind _tilesize_2 (Variables|Grid|GetTileSize))
  (return (+ (CallFunction|GetOrigin) (* (Math|Vector|GetRightVector (Variables|Default|GetScene)) (+ (* X (* _tilesize_2 2.0)) _tilesize_2)) (* (Math|Vector|GetForwardVector (Variables|Default|GetScene)) (+ (* Y (* _tilesize 2.0)) _tilesize)))))

(fn RetracePath
  (params (Target :type Path%20Tile%20Object%20Reference) (Start :type Path%20Tile%20Object%20Reference))
  (LocalVariables|SetCurrentTile Target)
  (while (not (== (LocalVariables|GetCurrentTile) Start))
    (Utilities|Array|AddUnique (LocalVariables|GetReversedPath) (LocalVariables|GetCurrentTile))
    (LocalVariables|SetCurrentTile (Variables|/Game/Blueprints/Pathfinding/PathTile.PathTile_C|GetPreviousTile (LocalVariables|GetCurrentTile))))
  (bind _arrayelement (Utilities|Array|ReverseforEachLoop (LocalVariables|GetReversedPath))
    (:LoopBody
      (Variables|/Game/Blueprints/Pathfinding/PathTile.PathTile_C|SetIs%20in%20Path _arrayelement true)
      (Utilities|Array|AddUnique (LocalVariables|GetOutPath) _arrayelement))
    (:Completed
      (Variables|Path|SetPath_ (LocalVariables|GetOutPath)))))

(fn TraceTile
  (params (Position :type Vector) (Channel :type ETraceTypeQuery%20Enum :default "TraceTypeQuery1"))
  (bind _returnvalue (Collision|SphereTraceByChannel Position Position (CallFunction|GetRealTileSize) Channel false 0 "None" true "(R=1.000000,G=0.000000,B=0.000000,A=1.000000)" "(R=0.000000,G=1.000000,B=0.000000,A=1.000000)" 2e+01))
  (return _returnvalue))

(fn IsValidPath
  (params (Path :type Array%20of%20Path%20Tile%20Object%20References))
  (return (> (Utilities|Array|Length Path) 0)))