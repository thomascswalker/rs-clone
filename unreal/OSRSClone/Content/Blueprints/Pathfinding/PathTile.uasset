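; A single grid tile actor for pathfinding, holding Walkable/Blocked type, G and H costs summed as F cost, and hover/select state.
; Hover and select events update state and call SetColor, which sets visibility from path, selection and hover, then pushes a material color.
; SetSwitchColors runs last, so type and path colors overwrite hover and selection highlights.
; Mouse event handlers are empty; their logic, which notifies the Grid, is disconnected.
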(event OnBeginCursorOver(StaticMesh)
  (params (TouchedComponent :type Primitive%20Component%20Object%20Reference))
  ;[1 1 1] Handle hovering
)

(event OnEndCursorOver(StaticMesh)
  (params (TouchedComponent :type Primitive%20Component%20Object%20Reference))
  ;[1 1 1] Handle hovering
)

(event OnReleased(StaticMesh)
  (params (TouchedComponent :type Primitive%20Component%20Object%20Reference) (ButtonReleased :type Key%20Structure :default "None"))
  ;[1 1 1] Handle selecting/deselecting tiles
)

(event Custom|SelectTile
  ;[1 1 1] Handle selecting/deselecting tiles
  (Variables|Default|SetSelected true)
  (CallFunction|SetColor))

(event Custom|DeselectTile
  ;[1 1 1] Handle selecting/deselecting tiles
  (Variables|Default|SetSelected false)
  (CallFunction|SetColor))

(event Custom|HoverTile
  ;[1 1 1] Handle hovering
  (Variables|Default|SetHovered true)
  (CallFunction|SetColor))

(event Custom|DehoverTile
  ;[1 1 1] Handle hovering
  (Variables|Default|SetHovered false)
  (CallFunction|SetColor))

(event EventBeginPlay
  (Utilities|FlowControl|Delay 0.2)
  (CallFunction|SetColor))

(event Collision|EventActorBeginOverlap
  (params (OtherActor :type Actor%20Object%20Reference)))

(event EventTick
  (params (DeltaSeconds :type Float%20%28single-precision%29)))

(fn ConstructionScript)

(fn SetColor
  (Utilities|FlowControl|Sequence
    (:then_0
      (CallFunction|OnHovered)
      (CallFunction|OnPath)
      (CallFunction|OnSelected)
      (CallFunction|SetSwitchColors))
    (:then_1
      (Rendering|Material|SetVectorParameterValueonMaterials (Variables|Default|GetStaticMesh) "Color" (Math|Conversions|ToVector(LinearColor) (Variables|Default|GetColor))))))

(fn GetFCost
  (return (+ (Variables|Default|GetGCost) (Variables|Default|GetHCost))))

(fn SetVisible
  (params (Override :type Boolean))
  (Rendering|SetVisibility (Variables|Default|GetStaticMesh) (Math|Boolean|ORBoolean Override (Variables|Default|GetSelected) (and (Variables|Default|GetHovered) (CallFunction|IsValidTile))) false))

(fn SetSwitchColors
  (switch Utilities|FlowControl|Switch|SwitchonPathTileTypes (Variables|Default|GetType)
    (:NewEnumerator1
      (if (CallFunction|IsinPath)
        (Variables|Default|SetColor "(R=1.000000,G=0.000000,B=0.807139,A=1.000000)")
        (else
          (Variables|Default|SetColor "(R=0.104527,G=1.000000,B=0.000000,A=1.000000)"))))
    (:NewEnumerator2
      (Variables|Default|SetColor "(R=1.000000,G=0.048397,B=0.000000,A=1.000000)"))))

(fn OnSelected
  (if (Variables|Default|GetSelected)
    (Variables|Default|SetColor "(R=0.000000,G=1.000000,B=0.983100,A=1.000000)")))

(fn OnPath
  (if (Utilities|Array|ContainsItem (Variables|/Game/Blueprints/Pathfinding/PathGrid.PathGrid_C|GetPath_ (Variables|Default|GetGrid)) self)
    (Variables|Default|SetColor "(R=1.000000,G=0.000000,B=0.807139,A=1.000000)")
    (CallFunction|SetVisible true)
    (else
      (CallFunction|SetSwitchColors)
      (CallFunction|SetVisible false))))

(fn IsinPath
  (return (Utilities|Array|ContainsItem (Variables|/Game/Blueprints/Pathfinding/PathGrid.PathGrid_C|GetPath_ (Variables|Default|GetGrid)) self)))

(fn OnHovered
  (if (Variables|Default|GetHovered)
    (Variables|Default|SetColor "(R=0.000000,G=1.000000,B=0.983100,A=1.000000)")))

(fn IsValidTile
  (return (Utilities|Enum|Equal(Enum) (Variables|Default|GetType) "NewEnumerator1")))