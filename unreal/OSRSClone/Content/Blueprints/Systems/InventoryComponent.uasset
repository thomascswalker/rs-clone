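; Inventory component that holds item structs in a Slots array and provides functions to write and add items.
; SetItem overwrites the slot at a given index with the supplied properties.
; AddItem finds the first slot with the same name as a stackable incoming item and replaces it through SetItem, without summing quantities.
; It returns false when nothing matches, with no empty-slot fallback.
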(event EventBeginPlay)

(event EventTick
  (params (DeltaSeconds :type Float%20%28single-precision%29)))

(fn SetItem
  (params (Index :type Integer) (Properties :type Item%20Properties%20Structure))
  (|SetBy-RefVar (Utilities|Array|Get(acopy) (Variables|Default|GetSlots) Index) Properties))

(fn AddItem
  (params (Properties :type Item%20Properties%20Structure))
  (LocalVariables|SetItem Properties)
  (for (_array_element _array_index) (Variables|Default|GetSlots)
    (LocalVariables|SetCurrentIndex _array_index)
    (if (and (Utilities|Enum|Equal(Enum) (.Name (Utilities|Struct|BreakItemProperties (LocalVariables|GetItem))) (.Name (Utilities|Struct|BreakItemProperties _array_element))) (.Stackable (Utilities|Struct|BreakItemProperties (LocalVariables|GetItem))))
      (CallFunction|SetItem (LocalVariables|GetCurrentIndex) (LocalVariables|GetItem))
      (return true)))
  (return false))