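; Inventory slot object that holds item data, a quantity and a selection state for an inventory component.
; Clearing resets the item and fires Changed, while select, deselect and toggle fire Selected or Deselected and debug-print the state.
; Drop finds the owning BP_InventoryComponent through the slot's Outer and passes itself to OnDrop.
; Examine only prints the item description.
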(event Custom|cleared
  (params (Task :type BP%20Task%20Object%20Reference))
  (Variables|Default|SetitemData (Utilities|Struct|MakeSItemData "None" false "/Game/Textures/Icons/blank.blank" 0 "" "(\"Drop\",\"Examine\")"))
  (Variables|Default|SethasItem false)
  (Variables|Default|Setquantity 0)
  (Default|CallChanged))

(event Custom|select
  (Variables|Default|SetisSelected true)
  (Default|CallSelected self)
  (Development|PrintString 0 (Utilities|String|ToString(Boolean) (Variables|Default|GetisSelected))))

(event Custom|deselect
  (Variables|Default|SetisSelected false)
  (Default|CallDeselected self)
  (Development|PrintString 0 (Utilities|String|ToString(Boolean) (Variables|Default|GetisSelected))))

(event Custom|toggleSelection
  (bind _self self)
  (bind _output_get (Variables|Default|SetisSelected (not (Variables|Default|GetisSelected))))
  (if _output_get
    (Default|CallSelected _self)
    (else
      (Default|CallDeselected _self)))
  (Development|PrintString 0 (Utilities|String|ToString(Boolean) (Variables|Default|GetisSelected))))

(fn GetInventory
  (bind _asbp_inventory_component (Utilities|Casting|CastToBP_InventoryComponent (Utilities|GetOuterObject self)))
  (return _asbp_inventory_component))

(fn ClearSlot
  (Variables|Default|SetitemData (Utilities|Struct|MakeSItemData "None" false "/Game/Textures/Icons/blank.blank" 0 "" "(\"Drop\",\"Examine\")"))
  (Variables|Default|SethasItem false)
  (Variables|Default|Setquantity 0)
  (Default|CallChanged))

(fn Drop
  (Default|OnDrop (CallFunction|GetInventory) self))

(fn Examine
  (Development|PrintString 0 (.description (Variables|Default|GetitemData))))