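; BP_InteractiveComponent is a component that gives its owning actor hover feedback and a list of interaction tasks.
; Its hover handlers toggle custom depth on the touched object and show or hide HUD text through BP_DefaultController's player character.
; The rich-text label joins the first task class's default display name with the owner's IInteractive name.
; Cursor-over binding is disconnected, and BeginPlay's interface check has no effect.
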(event Custom|OnHover
  (params (TouchedObject :type Primitive%20Component%20Object%20Reference))
  (CallFunction|UpdateHoverText true TouchedObject))

(event Custom|OnDehover
  (params (TouchedObject :type Primitive%20Component%20Object%20Reference))
  (CallFunction|UpdateHoverText false TouchedObject))

(event EventBeginPlay
  (if (Utilities|DoesObjectImplementInterface (Components|GetOwner) "/Game/Blueprints/Systems/Interaction/IInteractive.IInteractive_C")
    _))

(fn GetTask
  (params (Index :type Integer))
  (return (Utilities|Array|Get(acopy) (Variables|Default|GetTasks) Index)))

(fn UpdateHoverText
  (params (hovered :type Boolean) (object :type Primitive%20Component%20Object%20Reference))
  (Rendering|SetRenderCustomDepth object hovered)
  (bind _asbp_default_controller (Utilities|Casting|CastToBP_DefaultController (Game|GetPlayerController 0)))
  (bind _hud (Class|BPITaskExecutor|GetHud(Message) (Variables|/Game/Blueprints/Controllers/BP_DefaultController.BP_DefaultController_C|GetPlayerCharacter _asbp_default_controller)))
  (if hovered
    (Default|ShowHoverText _hud (CallFunction|GetHoverText))
    (else
      (Default|HideHoverText _hud))))

(fn GetHoverText
  ;[1 1 1] Object name
  (bind _asbpi_interactive (Utilities|Casting|CastToIInteractive (Components|GetOwner)))
  (bind _displayname (Default|GetDisplayName _asbpi_interactive))
  (return (Utilities|String|JoinStringArray (Utilities|Array|MakeArray (.DisplayName (Utilities|GetClassDefaults (Utilities|Array|Get(acopy) (Variables|Default|GetTasks)))) "<Item>" _displayname "</>") " ")))