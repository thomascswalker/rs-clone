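; BP_Interactive is an interactive actor with a highlightable mesh and an InteractiveComponent that holds its tasks.
; The construction script sets the mesh's custom depth stencil to 1 and copies Tasks from the InteractiveRow data table entry into the component.
; Getter functions expose the actor, display name, mesh and component.
; Cursor-over events are empty, and the custom-depth toggle based on Interactable is disconnected.
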(event MouseInput|EventActorBeginCursorOver)

(event MouseInput|EventActorEndCursorOver)

(fn ConstructionScript
  (bind _interactiverow (Variables|Default|GetInteractiveRow))
  (Rendering|SetCustomDepthStencilValue (Variables|Default|GetMesh) 1)
  (bind _returnvalue (Utilities|GetDataTableRow (.datatable _interactiverow) (.rowname _interactiverow))
    (:then
      (Variables|/Game/Blueprints/Systems/Interaction/BP_InteractiveComponent.BP_InteractiveComponent_C|SetTasks (Variables|Default|GetInteractiveComponent) (.Tasks (Utilities|Struct|BreakSInteractive _returnvalue))))))

(fn GetActor
  (return self))

(fn GetDisplayName
  (return (Utilities|GetDisplayName self)))

(fn GetHighlightableMesh
  (return (Variables|Default|GetMesh)))

(fn GetInteractiveComponent
  (return (Variables|Default|GetInteractiveComponent)))