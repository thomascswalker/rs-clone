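; BP_ResourceSpawn is a gatherable resource node that depletes and respawns, configured from a data table row.
; Construction caches the row and sets its mesh, and the display name comes from that data.
; Each gather randomly either signals that gathering can continue or depletes the node, with even odds.
; Depletion broadcasts an event, disables interaction and outline depth, swaps the mesh, and starts a timer that restores the node.
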(event Custom|Gathered
  (if (> (Math|Random|RandomFloat) 0.5)
    (CallFunction|Despawn)
    (else
      (Default|CallCanContinue))))

(event Custom|Despawn
  (bind _data (Variables|Default|GetData))
  (bind (_name _mesh _depletedmesh _gathermessage _gatherinterval _gatherchance _respawntime) (Utilities|Struct|BreakSResources _data))
  (Default|CallOnDepleted)
  (Variables|Default|SetDepleted? true)
  (Variables|Default|SetInteractable? false)
  (Components|StaticMesh|SetStaticMesh (Variables|Character|GetMesh) _depletedmesh)
  (Rendering|SetRenderCustomDepth (Variables|Character|GetMesh) false)
  (bind _returnvalue (Utilities|Time|SetTimerbyFunctionName self "Spawn" _respawntime))
  (Variables|Default|SetRespawnTimer _returnvalue))

(event Custom|Spawn
  (Utilities|IsValid self
    (:Is%20Valid
      (Variables|Default|SetDepleted? false)
      (Variables|Default|SetInteractable? true)
      (Components|StaticMesh|SetStaticMesh (Variables|Character|GetMesh) (.Mesh (Utilities|Struct|BreakSResources (Variables|Default|GetData)))))))

(fn ConstructionScript
  (bind _resource (Variables|Default|GetResource))
  (|CallParentFunction)
  (bind _returnvalue (Utilities|GetDataTableRow (.datatable _resource) (.rowname _resource))
    (:then
      (Variables|Default|SetData _returnvalue)
      (Components|StaticMesh|SetStaticMesh (Variables|Character|GetMesh) (.Mesh (Utilities|Struct|BreakSResources _returnvalue))))))

(fn GetDisplayName
  (return (Utilities|String|ToString(Name) (.name (Variables|Default|GetData)))))