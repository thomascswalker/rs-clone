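; BP_Item is a data-driven item actor that destroys itself when picked up.
; Its construction script calls the parent, binds to the PickedUp event, then looks up ItemRow in its data table to fill ItemData and set the static mesh.
; GetDisplayName returns the item name, appending the quantity in parentheses for stackable items.
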(event Custom|OnPickedUp
  (Actor|DestroyActor))

(fn ConstructionScript
  (bind _itemrow (Variables|Default|GetItemRow))
  (|CallParentFunction)
  (EventDispatchers|BindEventtoPickedUp (EventDispatchers|CreateEvent :!event Custom|OnPickedUp))
  (bind _returnvalue (Utilities|GetDataTableRow (.datatable _itemrow) (.rowname _itemrow))
    (:then
      (Variables|Default|SetItemData _returnvalue)
      (Components|StaticMesh|SetStaticMesh (Variables|Character|GetMesh) (.mesh (Variables|Default|GetItemData))))))

(fn GetDisplayName
  (bind _itemdata (Variables|Default|GetItemData))
  (bind _returnvalue (Utilities|String|ToString(Name) (.name _itemdata)))
  (if (.stackable _itemdata)
    (return (Utilities|String|JoinStringArray (Utilities|Array|MakeArray _returnvalue " (" (Utilities|String|ToString(Integer) (Variables|Default|GetQuantity)) ")") ""))
    (else
      (return _returnvalue))))