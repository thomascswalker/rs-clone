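; GenericObject is an interactive world actor whose available tasks come from a data table.
; Its construction script looks up the Row handle and, when found, copies that row's Tasks into the InteractiveComponent.
; It also sets the mesh's custom depth stencil to 1, and cursor hover toggles custom depth rendering on that mesh, allowing stencil-based highlighting.
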(event MouseInput|EventActorBeginCursorOver
  (Rendering|SetRenderCustomDepth (Variables|Default|GetMesh) true))

(event MouseInput|EventActorEndCursorOver
  (Rendering|SetRenderCustomDepth (Variables|Default|GetMesh) false))

(fn ConstructionScript
  (bind _row (Variables|Default|GetRow))
  (Rendering|SetCustomDepthStencilValue (Variables|Default|GetMesh) 1)
  (bind _returnvalue (Utilities|GetDataTableRow (.datatable _row) (.rowname _row))
    (:then
      (Variables|/Game/Blueprints/Tasks/InteractiveComponent.InteractiveComponent_C|SetTasks (Variables|Default|GetInteractiveComponent) (.Tasks (Utilities|Struct|BreakInteractiveData _returnvalue))))))