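; Task Blueprint with lifecycle events for initialization, start, end, completion and failure, apparently a skeleton for gameplay tasks.
; Completion and failure each broadcast an event dispatcher, passing the task itself to listeners.
; The other events hold only debug prints, except End, which is empty; the failure path also prints "Completed".
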(event Custom|Start
  (Development|PrintString 0 "Started"))

(event Custom|End)

(event Custom|TaskCompleted
  (Default|CallOnTaskCompleted self)
  (Development|PrintString 0 "Completed"))

(event Custom|TaskFailed
  (Default|CallOnTaskFailed self)
  (Development|PrintString 0 "Completed"))

(event Custom|Initialize
  (Development|PrintString 0 "Initialized"))