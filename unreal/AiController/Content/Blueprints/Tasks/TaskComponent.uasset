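; Task queue component that runs tasks sequentially on behalf of its TaskExecutor owner.
; New tasks are appended and initialized; priority tasks or an empty queue trigger SetCurrentTask, which always starts the head entry rather than the passed task.
; Completion or failure events drop the head and start the next task.
; Queue additions and removals are broadcast, and ClearQueue ends every task in reverse order.
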(event Custom|OnAddTaskToQueue
  (params (Task :type Task%20Object%20Reference))
  (CallFunction|AddTasktoQueue Task))

(event Custom|OnSetCurrentTask
  (params (Task :type Task%20Object%20Reference))
  (CallFunction|SetCurrentTask Task))

(event Custom|OnCurrentTaskCompleted
  (params (Task :type Task%20Object%20Reference))
  (CallFunction|TaskCompleted Task))

(event Custom|OnCurrentTaskFailed
  (params (Task :type Task%20Object%20Reference))
  (CallFunction|TaskCompleted Task))

(event Custom|OnCurrentTaskEnded
  (params (Task :type Task%20Object%20Reference))
  (CallFunction|TaskCompleted Task))

(fn AddTasktoQueue
  (params (Task :type Task%20Object%20Reference))
  (bind _astask_executor (Utilities|Casting|CastToTaskExecutor (Components|GetOwner)))
  (Variables|/Game/Blueprints/Tasks/Task.Task_C|SetTaskExecutor Task _astask_executor)
  (if (Variables|/Game/Blueprints/Tasks/Task.Task_C|GetPriority Task)
    (Utilities|Array|Add (Variables|Default|GetTaskList) Task :!label _label)
    (CallFunction|OnSetCurrentTask Task)
    (else
      (Utilities|IsQueueEmpty?
        (:Yes
          (goto _label))
        (:No
          (EventDispatchers|BindEventtoOnTaskFailed Task (EventDispatchers|CreateEvent :!event Custom|OnCurrentTaskFailed))
          (Default|Initialize Task)
          (Utilities|Array|Add (Variables|Default|GetTaskList) Task)
          (Default|CallTaskAddedtoQueue Task))))))

(fn RemoveTaskfromQueue
  (params (Task :type Task%20Object%20Reference))
  (bind _tasklist (Variables|Default|GetTaskList))
  (Utilities|Array|RemoveIndex _tasklist (Utilities|Array|FindItem _tasklist Task))
  (CallFunction|UnbindTask Task)
  (Default|CallTaskRemovedfromQueue Task))

(fn SetCurrentTask
  (params (Task :type Task%20Object%20Reference))
  (Variables|Default|SetSettingNewTask? true)
  (Default|CallTaskAddedtoQueue Task)
  (bind _astask_executor (Utilities|Casting|CastToTaskExecutor (Components|GetOwner))
    (:then
      (Utilities|IsQueueEmpty?
        (:Yes
          _)
        (:No
          (bind _output_get (LocalVariables|SetCurrentTask (Utilities|Array|Get(acopy) (Variables|Default|GetTaskList))))
          (CallFunction|UnbindTask _output_get)))
      (Variables|/Game/Blueprints/Tasks/Task.Task_C|SetTaskExecutor (LocalVariables|GetCurrentTask) _astask_executor)
      (CallFunction|BindTask (LocalVariables|GetCurrentTask))
      (Default|Initialize (LocalVariables|GetCurrentTask))
      (Default|Start (LocalVariables|GetCurrentTask))
      (Variables|Default|SetSettingNewTask? false))
    (:CastFailed
      (Variables|Default|SetSettingNewTask? false))))

(fn UnbindTask
  (params (Task :type Task%20Object%20Reference))
  (Utilities|IsValid Task
    (:Is%20Valid
      (EventDispatchers|UnbindEventfromOnTaskCompleted Task (EventDispatchers|CreateEvent :!event Custom|OnCurrentTaskCompleted))
      (EventDispatchers|UnbindEventfromOnTaskFailed Task (EventDispatchers|CreateEvent :!event Custom|OnCurrentTaskFailed)))))

(fn BindTask
  (params (Task :type Task%20Object%20Reference))
  (EventDispatchers|BindEventtoOnTaskCompleted Task (EventDispatchers|CreateEvent :!event Custom|OnCurrentTaskCompleted))
  (EventDispatchers|BindEventtoOnTaskFailed Task (EventDispatchers|CreateEvent :!event Custom|OnCurrentTaskFailed)))

(fn TaskCompleted
  (params (Task :type Task%20Object%20Reference))
  ;[1 1 1] Remove the current task from the queue
  (Utilities|Array|RemoveIndex (Variables|Default|GetTaskList))
  ;[1 1 1] Unbind the events from this task
  (CallFunction|UnbindTask Task)
  ;[1 1 1] If the queue is not empty, set the next task to the current task
  (Utilities|IsQueueEmpty?
    (:No
      (CallFunction|OnSetCurrentTask (Utilities|Array|Get(acopy) (Variables|Default|GetTaskList))))))

(fn ClearQueue
  (bind _arrayelement (Utilities|Array|ReverseforEachLoop (Variables|Default|GetTaskList))
    (:LoopBody
      (Default|End _arrayelement)
      (CallFunction|RemoveTaskfromQueue _arrayelement))))