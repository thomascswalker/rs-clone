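; Task blueprint that moves its executor's AI pawn to a Destination.
; On Start, it runs the parent logic, then issues an AI MoveTo through the executor's AI controller, accepting partial paths and tracking the goal continuously.
; Move results report completion or failure to the task, and End stops the controller's movement.
; The Move function is an empty stub.
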(event EventStart
  (|CallParentFunction)
  (bind _ai_controller (Default|GetAiController (Variables|Default|GetTaskExecutor)))
  (AI|AIMoveTo _ai_controller (Variables|Default|GetDestination) 0 5e+01 "Default" "Enable" true false true
    (:OnRequestFailed
      (CallFunction|TaskFailed))
    (:OnMoveFinished
      (CallFunction|TaskCompleted))))

(event EventEnd
  (bind _ai_controller (Default|GetAiController (Variables|Default|GetTaskExecutor)))
  (AI|Navigation|StopMovement _ai_controller))

(fn Move)