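; Player character that projects a decal onto the surface under the mouse cursor every tick, aligned to its normal.
; It spawns item pickups via a downward line trace and exposes getters for controllers, HUD, widgets and TaskComponent, with quest and skill getters empty.
; It acts as the "Player" dialogue participant with stubbed conditions, values and events.
; Progress bar and dialog widgets are created, but their viewport add and remove calls are unreachable.
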(event EventTick
  (params (DeltaSeconds :type Float%20%28single-precision%29))
  (bind _returnvalue (Game|GetPlayerController 0))
  (bind _hitresult (Game|Player|GetHitResultUnderCursorbyChannel _returnvalue "TraceTypeQuery1" true))
  (bind (_bblockinghit _binitialoverlap _time _distance _location _impactpoint _normal _impactnormal) (Collision|BreakHitResult _hitresult))
  (Transformation|SetWorldLocationAndRotation (Variables|Default|GetDecal) _location (Math|Rotator|MakeRotationfromAxes _impactnormal "0, 0, 0" "0, 0, 0") false false))

(fn ConstructionScript)

(fn SpawnItem
  (params (Item :type Item%20Data%20Structure) (Quantity :type Integer))
  (bind _returnvalue (Transformation|GetActorTransform))
  (bind (_x _y) (Math|Vector|BreakVector (.location _returnvalue)))
  (bind _outhit (Collision|LineTraceByChannel (.location _returnvalue) (Math|Vector|MakeVector _x _y -1e+04) "TraceTypeQuery1" false 0 "None"))
  (bind _returnvalue_2 (Game|SpawnActorfromClass "/Game/Blueprints/Systems/Items/Item.Item_C" (Math|Transform|MakeTransform (.Location (Collision|BreakHitResult _outhit)) "0, 0, 0" "1,1,1") "AdjustIfPossibleButAlwaysSpawn" 0 (Utilities|Struct|MakeDataTableRowHandle "/Game/Blueprints/Systems/Items/ItemTable.ItemTable" (.Name (Utilities|Struct|BreakItemData Item))) Quantity (Utilities|Struct|MakeDataTableRowHandle "/Game/Blueprints/Systems/Interaction/InteractiveTable.InteractiveTable" "Pickup") true 0))
  (return (Utilities|IsValid _returnvalue_2)))

(fn ConstructProgressBar
  (params (Task :type Task%20Object%20Reference))
  (UserInterface|CreateWidget "/Game/Blueprints/Systems/Tasks/TaskProgressWidget.TaskProgressWidget_C" 0 (Variables|/Game/Blueprints/Systems/Tasks/Task.Task_C|GetProgressMessage Task) (Variables|/Game/Blueprints/Systems/Tasks/Task.Task_C|GetProgressTime Task)))

(fn DestroyProgressBar
  (Utilities|IsValid 0))

(fn ConstructDialogWidget
  (params (Task :type Dialog%20Task%20Object%20Reference) (Dialog :type Dlg%20Dialogue%20Object%20Reference))
  (bind _returnvalue (Class|DlgManager|StartDialoguewithDefaultParticipants Dialog))
  (UserInterface|CreateWidget "/Game/Blueprints/Systems/Dialog/DialogWidget.DialogWidget_C" 0 Task _returnvalue))

(fn DestroyDialogWidget
  (Utilities|IsValid 0))

(fn GetPlayerController
  (bind _asrscontroller (Utilities|Casting|CastToRSController (Game|GetPlayerController 0)))
  (return _asrscontroller))

(fn CheckCondition
  (params (Context :type Dlg%20Context%20Object%20Reference) (ConditionName :type Name :default "None"))
  (return false))

(fn GetAiController
  (return (AI|GetAIController self)))

(fn GetBoolValue
  (params (ValueName :type Name :default "None"))
  (return false))

(fn GetCharacter
  (return self))

(fn GetFloatValue
  (params (ValueName :type Name :default "None"))
  (return 0.0))

(fn GetHud
  (bind _foundwidgets (Widget|GetAllWidgetsOfClass "/Game/Blueprints/Systems/Interface/HUD.HUD_C" false))
  (for _array_element _foundwidgets
    (return _array_element)))

(fn GetIntValue
  (params (ValueName :type Name :default "None"))
  (return 0))

(fn GetNameValue
  (params (ValueName :type Name :default "None"))
  (return "None"))

(fn GetParticipantDisplayName
  (params (ActiveSpeaker :type Name :default "None"))
  (return "Player"))

(fn GetParticipantGender
  (return "Masculine"))

(fn GetParticipantIcon
  (params (ActiveSpeaker :type Name :default "None") (ActiveSpeakerState :type Name :default "None"))
  (return 0))

(fn GetParticipantName
  (return "Player"))

(fn GetProgressBar
  (return 0))

(fn GetQuestComponent
  (return 0))

(fn GetSkillComponent
  (return 0))

(fn GetTaskComponent
  (return (Variables|Default|GetTaskComponent)))

(fn GetWidget
  (params (Widget :type User%20Widget%20Class%20Reference))
  (bind _foundwidgets (Widget|GetAllWidgetsOfClass Widget true))
  (for _array_element _foundwidgets
    (return _array_element)))

(fn ModifyBoolValue
  (params (ValueName :type Name :default "None") (bNewValue :type Boolean))
  (return false))

(fn ModifyFloatValue
  (params (ValueName :type Name :default "None") (bDelta :type Boolean) (Value :type Float%20%28single-precision%29))
  (return false))

(fn ModifyIntValue
  (params (ValueName :type Name :default "None") (bDelta :type Boolean) (Value :type Integer))
  (return false))

(fn ModifyNameValue
  (params (ValueName :type Name :default "None") (NameValue :type Name :default "None"))
  (return false))

(fn OnDialogueEvent
  (params (Context :type Dlg%20Context%20Object%20Reference) (EventName :type Name :default "None"))
  (return false))