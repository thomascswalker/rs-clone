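; RSBaseCharacter is a base character for a click-style game with item pickups and timed tasks, exposing its skill and task components, AI controller and widgets through getters.
; Each tick it moves a decal to the surface under the player's cursor, aligned to the impact normal.
; SpawnItem traces down to the ground and spawns a data-table-driven pickup there.
; Task progress bars are created from task data and removed on demand.
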(event EventTick
  (params (DeltaSeconds :type Float%20%28single-precision%29))
  (bind _returnvalue (Game|GetPlayerController 0))
  (bind _hitresult (Game|Player|GetHitResultUnderCursorbyChannel _returnvalue "TraceTypeQuery1" true))
  (bind (_bblockinghit _binitialoverlap _time _distance _location _impactpoint _normal _impactnormal) (Collision|BreakHitResult _hitresult))
  (Transformation|SetWorldLocationAndRotation (Variables|Default|GetDecal) _location (Math|Rotator|MakeRotationfromAxes _impactnormal "0, 0, 0" "0, 0, 0") false false))

(fn ConstructionScript)

(fn SpawnItem
  (params (Item :type Item%20Data%20Structure) (Quantity :type Integer))
  (bind _returnvalue (Transformation|GetActorTransform))
  (bind (_x _y) (Math|Vector|BreakVector (.location _returnvalue)))
  (bind _outhit (Collision|LineTraceByChannel (.location _returnvalue) (Math|Vector|MakeVector _x _y -1e+04) "TraceTypeQuery1" false 0 "None"))
  (bind _returnvalue_2 (Game|SpawnActorfromClass "/Game/Blueprints/Systems/Items/Item.Item_C" (Math|Transform|MakeTransform (.Location (Collision|BreakHitResult _outhit)) "0, 0, 0" "1,1,1") "AdjustIfPossibleButAlwaysSpawn" 0 (Utilities|Struct|MakeDataTableRowHandle "/Game/Blueprints/Systems/Items/ItemTable.ItemTable" (.Name (Utilities|Struct|BreakItemData Item))) Quantity (Utilities|Struct|MakeDataTableRowHandle "/Game/Blueprints/Systems/Interaction/InteractiveTable.InteractiveTable" "Pickup") true 0))
  (return (Utilities|IsValid _returnvalue_2)))

(fn ConstructProgressBar
  (params (Task :type Task%20Object%20Reference))
  (bind _returnvalue (UserInterface|CreateWidget "/Game/Blueprints/Systems/Interface/TaskProgressWidget.TaskProgressWidget_C" 0 (Variables|/Game/Blueprints/Systems/Tasks/Task.Task_C|GetProgressMessage Task) (Variables|/Game/Blueprints/Systems/Tasks/Task.Task_C|GetProgressTime Task)))
  (bind _output_get (Variables|Default|SetProgressBarWidget _returnvalue))
  (UserInterface|Viewport|AddtoViewport _output_get 0)
  (return _output_get))

(fn DestroyProgressBar
  (Utilities|IsValid (Variables|Default|GetProgressBarWidget)
    (:Is%20Valid
      (Widget|RemovefromParent (Variables|Default|GetProgressBarWidget)))))

(fn GetAiController
  (return (AI|GetAIController self)))

(fn GetCharacter
  (return self))

(fn GetProgressBar
  (return (Variables|Default|GetProgressBarWidget)))

(fn GetSkillComponent
  (return (Variables|Default|GetSkillComponent)))

(fn GetTaskComponent
  (return (Variables|Default|GetTaskComponent)))

(fn GetWidget
  (params (Widget :type User%20Widget%20Class%20Reference))
  (bind _foundwidgets (Widget|GetAllWidgetsOfClass Widget true))
  (for _array_element _foundwidgets
    (return _array_element)))