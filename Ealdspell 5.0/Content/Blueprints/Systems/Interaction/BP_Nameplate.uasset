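; Nameplate actor that shows an interactive object's name and health through a WBP_Nameplate widget component, turned toward the player camera every Tick.
; On BeginPlay it sets the name text from the InteractiveComponent's data and binds to the CombatComponent's value-changed event to forward health updates to the widget.
; SetCombatBars, run from the construction script, is a stub that only prints a debug string when a CombatComponent is valid.
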(event Custom|CustomEvent_0
  (params (Component :type BP%20Combat%20Component%20Object%20Reference))
  (bind _aswbp_nameplate (Utilities|Casting|CastToWBP_Nameplate (UserInterface|GetWidget (Variables|Default|GetWidgetComponent))))
  (Default|HealthUpdated _aswbp_nameplate Component))

(event EventBeginPlay
  (CallFunction|SetName)
  (EventDispatchers|BindEventtoValueChanged (Variables|Default|GetCombatComponent) (EventDispatchers|CreateEvent :!event Custom|CustomEvent_0)))

(event EventTick
  (params (DeltaSeconds :type Float%20%28single-precision%29))
  (Transformation|SetWorldRotation (Variables|Default|GetWidgetComponent) (Math|Rotator|FindLookatRotation (Transformation|GetActorLocation) (Transformation|GetActorLocation (Game|GetPlayerCameraManager 0))) false false))

(fn ConstructionScript
  (CallFunction|SetCombatBars))

(fn SetName
  (bind _interactivecomponent (Variables|Default|GetInteractiveComponent))
  (Utilities|IsValid _interactivecomponent
    (:Is%20Valid
      (bind _aswbp_nameplate (Utilities|Casting|CastToWBP_Nameplate (UserInterface|GetWidget (Variables|Default|GetWidgetComponent))))
      (Rendering|Components|TextRender|SetText (Variables|/Game/Blueprints/Systems/Interface/WBP_Nameplate.WBP_Nameplate_C|GetTextName _aswbp_nameplate) (Utilities|Text|ToText(Name) (.name (Variables|/Game/Blueprints/Systems/Interaction/BP_InteractiveComponent.BP_InteractiveComponent_C|GetData _interactivecomponent)))))))

(fn SetCombatBars
  (Utilities|IsValid (Variables|Default|GetCombatComponent)
    (:Is%20Valid
      (Development|PrintString "Hello"))))