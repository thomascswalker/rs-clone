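; Component that makes an IInteractive owner highlightable on cursor hover, with an outline and a HUD prompt.
; On BeginPlay it binds cursor-over events on the owner's highlightable mesh and creates an outline material colored by interaction Type.
; Hover toggles the mesh's custom depth and shows or hides rich text built from the first task's name and owner's display name.
; The outline color is applied by setting the player camera's post-process materials on hover.
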(event Custom|OnHover
  (params (TouchedObject :type Primitive%20Component%20Object%20Reference))
  (CallFunction|UpdateHoverText true TouchedObject)
  (CallFunction|UpdateHoverColor))

(event Custom|OnDehover
  (params (TouchedObject :type Primitive%20Component%20Object%20Reference))
  (CallFunction|UpdateHoverText false TouchedObject))

(event EventBeginPlay
  (CallFunction|Initialize))

(fn GetTask
  (params (Index :type Integer))
  (return (Utilities|Array|Get(acopy) (Variables|Default|GetTasks) Index)))

(fn UpdateHoverText
  (params (hovered :type Boolean) (object :type Primitive%20Component%20Object%20Reference))
  (Rendering|SetRenderCustomDepth object hovered)
  (bind _asbp_default_controller (Utilities|Casting|CastToBP_DefaultController (Game|GetPlayerController 0)))
  (bind _hud (Class|BPITaskExecutor|GetHud(Message) (Variables|/Game/Blueprints/Controllers/BP_DefaultController.BP_DefaultController_C|GetPlayerCharacter _asbp_default_controller)))
  (if hovered
    (Default|ShowHoverText _hud (CallFunction|GetHoverText))
    (else
      (Default|HideHoverText _hud))))

(fn GetHoverText
  ;[1 1 1] Object name
  (bind _asiinteractive (Utilities|Casting|CastToIInteractive (Components|GetOwner)))
  (bind _displayname (Default|GetDisplayName _asiinteractive))
  (return (Utilities|String|JoinStringArray (Utilities|Array|MakeArray (.DisplayName (Utilities|GetClassDefaults (Utilities|Array|Get(acopy) (Variables|Default|GetTasks)))) "<Item>" _displayname "</>") " ")))

(fn Initialize
  (if (Utilities|DoesObjectImplementInterface (Components|GetOwner) "/Game/Blueprints/Systems/Interaction/IInteractive.IInteractive_C")
    (bind _asiinteractive (Utilities|Casting|CastToIInteractive (Components|GetOwner)))
    (bind _mesh (Default|GetHighlightableMesh _asiinteractive))
    ;[1 1 1] Bind interactive events
    (EventDispatchers|BindEventtoOnBeginCursorOver _mesh (EventDispatchers|CreateEvent :!event Custom|OnHover))
    (EventDispatchers|BindEventtoOnEndCursorOver _mesh (EventDispatchers|CreateEvent :!event Custom|OnDehover))
    (Rendering|SetRenderCustomDepth _mesh false)
    (Rendering|SetCustomDepthStencilValue _mesh 1)
    ;[1 1 1] Set hover color
    (bind _returnvalue (Rendering|Material|CreateDynamicMaterialInstance "/Game/Materials/M_OutlineInstance.M_OutlineInstance" "None" "None" :!class /Script/Engine.KismetMaterialLibrary))
    (switch Utilities|FlowControl|Switch|SwitchonEInteractiveTypes (Variables|Default|GetType)
      (:NewEnumerator0
        (Rendering|Material|SetVectorParameterValue _returnvalue "Color" "(R=0.000000,G=0.377165,B=0.502887,A=1.000000)" :!class /Script/Engine.MaterialInstanceDynamic))
      (:NewEnumerator1
        (Rendering|Material|SetVectorParameterValue _returnvalue "Color" "(R=0.309804,G=0.501961,B=0.000000,A=1.000000)" :!class /Script/Engine.MaterialInstanceDynamic))
      (:NewEnumerator2
        (Rendering|Material|SetVectorParameterValue _returnvalue "Color" "(R=0.500000,G=0.275000,B=0.000000,A=1.000000)" :!class /Script/Engine.MaterialInstanceDynamic))
      (:NewEnumerator3
        (Rendering|Material|SetVectorParameterValue _returnvalue "Color" "(R=0.500000,G=0.500000,B=0.000000,A=1.000000)" :!class /Script/Engine.MaterialInstanceDynamic))
      (:NewEnumerator4
        (Rendering|Material|SetVectorParameterValue _returnvalue "Color" "(R=0.500000,G=0.000000,B=0.000000,A=1.000000)" :!class /Script/Engine.MaterialInstanceDynamic)))
    (Variables|Default|SetOutlineMaterial _returnvalue)))

(fn UpdateHoverColor
  (bind _asbp_default_controller (Utilities|Casting|CastToBP_DefaultController (Game|GetPlayerController 0)))
  (Utilities|Struct|SetmembersinPostProcessSettings (Variables|/Script/Engine.CameraComponent|GetPostProcessSettings (Variables|/Game/Blueprints/Controllers/BP_DefaultPlayerCharacter.BP_DefaultPlayerCharacter_C|GetCamera (Variables|/Game/Blueprints/Controllers/BP_DefaultController.BP_DefaultController_C|GetPlayerCharacter _asbp_default_controller))) (Utilities|Struct|MakeWeightedBlendables (Utilities|Array|MakeArray (Utilities|Struct|MakeWeightedBlendable 1.0 (Variables|Default|GetOutlineMaterial))))))