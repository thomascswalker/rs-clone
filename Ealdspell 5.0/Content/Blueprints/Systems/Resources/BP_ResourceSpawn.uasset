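; BP_ResourceSpawn is a gatherable, respawning resource node configured from a data table row.
; The construction script loads that row, sets the mesh and fills the interactive component with the resource name and gather task.
; Each gather randomly either depletes the node or signals that gathering can continue.
; Depletion notifies listeners, swaps to the depleted mesh, disables custom depth and starts a timer that restores the node.
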(event Custom|Gathered
  (if (> (Math|Random|RandomFloat) 0.5)
    (CallFunction|Despawn)
    (else
      (Default|CallCanContinue))))

(event Custom|Despawn
  (Default|CallOnDepleted)
  (Variables|Default|SetIsDepleted true)
  (Components|StaticMesh|SetStaticMesh (Variables|Default|GetMesh) (.depletedmesh (Variables|Default|GetResourceData)))
  (Rendering|SetRenderCustomDepth (Variables|Default|GetMesh) false)
  (bind _returnvalue (Utilities|Time|SetTimerbyFunctionName self "Spawn" (.respawntime (Variables|Default|GetResourceData))))
  (Variables|Default|SetRespawnTimer _returnvalue))

(event Custom|Spawn
  (Utilities|IsValid self
    (:Is%20Valid
      (Variables|Default|SetIsDepleted false)
      (Components|StaticMesh|SetStaticMesh (Variables|Default|GetMesh) (.mesh (Variables|Default|GetResourceData)))
      (Utilities|Time|InvalidateTimerHandle (Variables|Default|GetRespawnTimer)))))

(fn ConstructionScript
  (bind _resource (Variables|Default|GetResource))
  (|CallParentFunction)
  (bind _returnvalue (Utilities|GetDataTableRow (.datatable _resource) (.rowname _resource))
    (:then
      (bind _output_get (Variables|Default|SetResourceData _returnvalue))
      (Components|StaticMesh|SetStaticMesh (Variables|Default|GetMesh) (.mesh _output_get))
      (Variables|/Game/Blueprints/Systems/Interaction/BP_InteractiveComponent.BP_InteractiveComponent_C|SetData (Variables|Default|GetBP_InteractiveComponent) (Utilities|Struct|MakeSInteractive (.name _output_get) (Utilities|Array|MakeArray "/Game/Blueprints/Systems/Resources/BPT_GatherResource.BPT_GatherResource_C") "NewEnumerator2")))))

(fn GetDisplayName
  (return (Utilities|String|ToString(Name) "None")))