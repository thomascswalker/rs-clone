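; BP_Task is a task object that a TaskExecutor holds in its task component's queue, tracking its state from queued or active to completed, failed or ended.
; End, completion and failure events fire matching dispatchers, and CanContinue allows only active or queued tasks.
; Helpers add or remove it in task UI, clear the progress bar, dequeue it, or requeue a fresh same-class copy carrying over its main properties.
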(event Custom|Start
  (Variables|Default|SetState "NewEnumerator1"))

(event Custom|TaskEnded
  (Default|CallOnTaskEnded self)
  (Variables|Default|SetState "NewEnumerator4"))

(event Custom|TaskCompleted
  (Default|CallOnTaskCompleted self)
  (Variables|Default|SetState "NewEnumerator2"))

(event Custom|TaskFailed
  (Default|CallOnTaskFailed self)
  (Variables|Default|SetState "NewEnumerator3"))

(event Custom|Initialize
  (Variables|Default|SetState "NewEnumerator0"))

(fn GetDebugMessage
  (params (Status :type String))
  (return (Utilities|String|Append (Utilities|GetObjectName self) " " Status)))

(fn AddDisplayTask
  (bind _task_component (Default|GetTaskComponent (Variables|Default|GetTaskExecutor)))
  (Default|AddItem (Variables|/Game/Blueprints/Systems/Tasks/BP_TaskComponent.BP_TaskComponent_C|GetWidget _task_component) self))

(fn RemoveDisplayTask
  (bind _widgetfound (Default|GetWidget (Variables|Default|GetTaskExecutor) "/Game/Blueprints/Systems/Tasks/WBP_TaskWindow.WBP_TaskWindow_C"))
  (bind _aswbp_task_window (Utilities|Casting|CastToWBP_TaskWindow _widgetfound))
  (Default|RemoveItem _aswbp_task_window self))

(fn CanContinue
  (switch Utilities|FlowControl|Switch|SwitchonETaskStates (Variables|Default|GetState)
    (:NewEnumerator0
      _)
    (:NewEnumerator1
      _)
    (:NewEnumerator2
      (return false))
    (:NewEnumerator3
      (return false))
    (:NewEnumerator4
      (return false)))
  (return true))

(fn GetThisTaskinExecutor
  (bind _task_component (Default|GetTaskComponent (Variables|Default|GetTaskExecutor)))
  (return (Utilities|Array|Get(acopy) (Variables|/Game/Blueprints/Systems/Tasks/BP_TaskComponent.BP_TaskComponent_C|GetTaskList _task_component) (Utilities|Array|FindItem (Variables|/Game/Blueprints/Systems/Tasks/BP_TaskComponent.BP_TaskComponent_C|GetTaskList _task_component) self))))

(fn DestroyProgressBar
  (bind _widgetfound (Default|GetWidget (Variables|Default|GetTaskExecutor) "/Game/Blueprints/Systems/Tasks/WBP_TaskProgress.WBP_TaskProgress_C"))
  (Widget|RemovefromParent _widgetfound))

(fn RequeueCopy
  (bind _returnvalue (CallFunction|GetCopy))
  (bind _task_component (Default|GetTaskComponent (Variables|Default|GetTaskExecutor)))
  (Default|AddTasktoQueue _task_component _returnvalue))

(fn GetCopy
  (bind _self self)
  (bind _returnvalue (Game|ConstructObjectfromClass (Utilities|GetOuterObject _self) (Utilities|GetClass _self) (Variables|Default|GetInstigator) (Variables|Default|GetActor) (Variables|Default|GetIsPriority) (Variables|Default|GetIsRequired)))
  (return _returnvalue))

(fn Next
  (bind _task_component (Default|GetTaskComponent (Variables|Default|GetTaskExecutor)))
  (Default|RemoveTaskfromQueue _task_component self))