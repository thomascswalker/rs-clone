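; Task queue component for owners implementing BPI_TaskExecutor, which also opens a "Tasks" panel on BeginPlay.
; Priority tasks, or tasks added to an empty queue, start at once; others are initialized and wait.
; Setting a current task ends the first listed task and resets the list to the new one, with SettingNewTask guarding the swap.
; Completion and failure events advance the queue, while a failed required task ends all listed tasks.
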(event Custom|OnAddTaskToQueue
  (params (Task :type BP%20Task%20Object%20Reference))
  (CallFunction|AddTasktoQueue Task)
  (Default|AddDisplayTask Task))

(event Custom|OnSetCurrentTask
  (params (Task :type BP%20Task%20Object%20Reference))
  (CallFunction|SetCurrentTask Task))

(event Custom|OnCurrentTaskCompleted
  (params (Task :type BP%20Task%20Object%20Reference))
  (CallFunction|CompleteTask Task))

(event Custom|OnCurrentTaskFailed
  (params (Task :type BP%20Task%20Object%20Reference))
  (CallFunction|FailTask Task))

(event Custom|OnCurrentTaskEnded
  (params (Task :type BP%20Task%20Object%20Reference))
  (CallFunction|EndTask Task))

(event Custom|Show
  (bind _returnvalue (UserInterface|CreateWidget "/Game/Blueprints/Systems/Tasks/WBP_TaskWindow.WBP_TaskWindow_C"))
  (bind _output_get (Variables|Default|SetWidget _returnvalue))
  (bind _returnvalue_2 (UserInterface|CreateWidget "/Game/Blueprints/Systems/Interface/WBP_PanelTitleBar.WBP_PanelTitleBar_C" 0 "Tasks" _output_get))
  (UserInterface|Viewport|AddtoViewport _returnvalue_2 0))

(event EventBeginPlay
  (CallFunction|Show))

(fn AddTasktoQueue
  (params (Task :type BP%20Task%20Object%20Reference))
  (bind _asbpi_task_executor (Utilities|Casting|CastToBPI_TaskExecutor (Components|GetOwner)))
  (Variables|/Game/Blueprints/Systems/Tasks/BP_Task.BP_Task_C|SetTaskExecutor Task _asbpi_task_executor)
  (if (Variables|/Game/Blueprints/Systems/Tasks/BP_Task.BP_Task_C|GetIsPriority Task)
    (Utilities|Array|Add (Variables|Default|GetTaskList) Task :!label _label)
    (CallFunction|OnSetCurrentTask Task)
    (else
      (Utilities|IsQueueEmpty?
        (:Yes
          (goto _label))
        (:No
          (CallFunction|UnbindTask Task)
          (Default|Initialize Task)
          (Utilities|Array|Add (Variables|Default|GetTaskList) Task)
          (Default|CallTaskAddedtoQueue Task)
          (Variables|/Game/Blueprints/Systems/Tasks/BP_Task.BP_Task_C|SetState Task "NewEnumerator1"))))))

(fn BindTask
  (params (Task :type BP%20Task%20Object%20Reference))
  (EventDispatchers|BindEventtoOnTaskCompleted Task (EventDispatchers|CreateEvent :!event Custom|OnCurrentTaskCompleted))
  (EventDispatchers|BindEventtoOnTaskFailed Task (EventDispatchers|CreateEvent :!event Custom|OnCurrentTaskFailed)))

(fn ClearQueue
  (for _array_element (Variables|Default|GetTaskList)
    (Default|TaskEnded _array_element)))

(fn CompleteTask
  (params (Task :type BP%20Task%20Object%20Reference))
  ;[1 1 1] Remove the current task from the queue
  (Utilities|Array|RemoveIndex (Variables|Default|GetTaskList))
  ;[1 1 1] Unbind the events from this task
  (CallFunction|UnbindTask Task)
  ;[1 1 1] If the queue is not empty, set the next task to the current task
  (Utilities|IsQueueEmpty?
    (:No
      (bind _task (CallFunction|GetFirstTask))
      (CallFunction|OnSetCurrentTask _task))))

(fn EndTask
  (params (Task :type BP%20Task%20Object%20Reference))
  (bind _tasklist (Variables|Default|GetTaskList))
  (Utilities|Array|RemoveIndex _tasklist (Utilities|Array|FindItem _tasklist Task))
  (if (not (Variables|Default|GetSettingNewTask?))
    (Utilities|IsQueueEmpty?
      (:No
        (bind _task (CallFunction|GetFirstTask))
        (EventDispatchers|UnbindEventfromOnTaskFailed _task (EventDispatchers|CreateEvent :!event RemoveTaskfromQueue))
        (EventDispatchers|UnbindEventfromOnTaskCompleted _task (EventDispatchers|CreateEvent :!event Custom|OnCurrentTaskCompleted))
        (EventDispatchers|UnbindEventfromOnTaskFailed _task (EventDispatchers|CreateEvent :!event Custom|OnCurrentTaskFailed))
        (Default|Start _task)))))

(fn FailTask
  (params (Task :type BP%20Task%20Object%20Reference))
  (Default|CallTaskRemovedfromQueue Task)
  (if (Variables|/Game/Blueprints/Systems/Tasks/BP_Task.BP_Task_C|GetIsRequired Task)
    (CallFunction|ClearQueue)
    (else
      (CallFunction|OnCurrentTaskEnded Task))))

(fn GetFirstTask
  (for (_array_element _array_index) (Variables|Default|GetTaskList)
    (if (== _array_index 0)
      (return _array_element))))

(fn RemoveTaskfromQueue
  (params (Task :type BP%20Task%20Object%20Reference))
  (if (not (Variables|Default|GetSettingNewTask?))
    (Default|CallTaskRemovedfromQueue Task)
    (CallFunction|EndTask Task)
    (CallFunction|UnbindTask Task)
    (Utilities|Array|RemoveItem (Variables|Default|GetTaskList) Task)))

(fn SetCurrentTask
  (params (Task :type BP%20Task%20Object%20Reference))
  (Variables|Default|SetSettingNewTask? true)
  (Default|CallTaskAddedtoQueue Task)
  (bind _asbpi_task_executor (Utilities|Casting|CastToBPI_TaskExecutor (Components|GetOwner))
    (:then
      (Utilities|IsQueueEmpty?
        (:Yes
          _)
        (:No
          (bind _task (CallFunction|GetFirstTask))
          (bind _output_get (LocalVariables|SetCurrentTask _task))
          (CallFunction|UnbindTask _output_get)
          (bind _task_2 (CallFunction|GetFirstTask))
          (Default|TaskEnded _task_2)
          (Utilities|Array|Clear (Variables|Default|GetTaskList))
          (Utilities|Array|Add (Variables|Default|GetTaskList) Task)))
      (Variables|/Game/Blueprints/Systems/Tasks/BP_Task.BP_Task_C|SetTaskExecutor Task _asbpi_task_executor)
      (CallFunction|BindTask Task)
      (Default|Initialize Task)
      (Default|Start Task)
      (Variables|Default|SetSettingNewTask? false))
    (:CastFailed
      (Variables|Default|SetSettingNewTask? false))))

(fn UnbindTask
  (params (Task :type BP%20Task%20Object%20Reference))
  (Utilities|IsValid Task
    (:Is%20Valid
      (EventDispatchers|UnbindEventfromOnTaskCompleted Task (EventDispatchers|CreateEvent :!event Custom|OnCurrentTaskCompleted))
      (EventDispatchers|UnbindEventfromOnTaskFailed Task (EventDispatchers|CreateEvent :!event Custom|OnCurrentTaskFailed)))))