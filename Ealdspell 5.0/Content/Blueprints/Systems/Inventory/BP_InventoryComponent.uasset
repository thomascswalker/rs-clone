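; Player inventory component that holds a fixed number of slot objects and shows them in a toggleable widget, opened on BeginPlay.
; Pickups stack by item name or take the first empty slot, then fire change events or report a full inventory.
; Drops are queued as tasks on the player character's task component, and helpers handle slot deselection.
; HasItem is unfinished, returning true whenever any slot exists.
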(event Custom|OnPickup
  (params (Item :type S%20Item%20Data%20Structure) (Quantity :type Integer) (Actor :type Actor%20Object%20Reference))
  (bind _added (CallFunction|AddtoInventory Item Quantity))
  (if _added
    (bind _asbp_item (Utilities|Casting|CastToBP_Item Actor))
    (Default|CallPickedUp _asbp_item)))

(event Custom|OnDrop
  (params (Slot :type BP%20Inventory%20Slot%20Object%20Reference))
  (bind _returnvalue (Game|ConstructObjectfromClass "/Game/Blueprints/Systems/Items/BPT_DropItem.BPT_DropItem_C" (CallFunction|GetTaskComponent) (Variables|/Game/Blueprints/Systems/Inventory/BP_InventorySlot.BP_InventorySlot_C|GetitemData Slot) (Variables|/Game/Blueprints/Systems/Inventory/BP_InventorySlot.BP_InventorySlot_C|Getquantity Slot) 0))
  (EventDispatchers|BindEventtoOnTaskCompleted _returnvalue (EventDispatchers|CreateEvent Slot :!event Cleared))
  (Default|OnAddTasktoQueue (CallFunction|GetTaskComponent) _returnvalue))

(event Custom|OnAdd
  (params (Item :type S%20Item%20Data%20Structure))
  (CallFunction|AddtoInventory Item))

(event Custom|OnDeselectAll
  (for _array_element (Variables|Default|Get_items)
    (Default|Deselect _array_element)))

(event Custom|OnDeselectAllExcept
  (params (slot :type BP%20Inventory%20Slot%20Object%20Reference))
  (for _array_element (Variables|Default|Get_items)
    (if (!= slot _array_element)
      (Default|Deselect _array_element))))

(event EventBeginPlay
  (CallFunction|Initialize)
  (CallFunction|Show))

(event EventShow
  (Utilities|IsValid (Variables|Default|Get_widget)
    (:Is%20Valid
      _)
    (:Is%20Not%20Valid
      (bind _returnvalue (UserInterface|CreateWidget "/Game/Blueprints/Systems/Inventory/WBP_Inventory.WBP_Inventory_C" 0 self))
      (Variables|Default|Set_widget _returnvalue)))
  (UserInterface|Viewport|AddtoViewport (Variables|Default|Get_widget) 0)
  (Variables|Default|Set_visible true)
  (Default|CallShowEvent))

(event EventHide
  (bind __widget (Variables|Default|Get_widget))
  (Utilities|IsValid __widget
    (:Is%20Valid
      (Widget|RemovefromParent __widget))
    (:Is%20Not%20Valid
      _))
  (Variables|Default|Set_visible false)
  (Default|CallCloseEvent))

(event EventToggle
  (if (not (Variables|Default|Get_visible))
    (CallFunction|Show)
    (else
      (CallFunction|Hide))))

(fn GetTaskComponent
  (bind _asbp_default_player_character (Utilities|Casting|CastToBP_DefaultPlayerCharacter (Components|GetOwner)))
  (return (Variables|/Game/Blueprints/Controllers/BP_DefaultPlayerCharacter.BP_DefaultPlayerCharacter_C|GetTaskComponent _asbp_default_player_character)))

(fn Initialize
  (for _index (range 0 (- (Variables|Default|Get_maxSlots) 1))
    (bind _returnvalue (Game|ConstructObjectfromClass "/Game/Blueprints/Systems/Inventory/BP_InventorySlot.BP_InventorySlot_C" self))
    (Utilities|Array|Add (Variables|Default|Get_items) _returnvalue)
    (EventDispatchers|BindEventtoSelected _returnvalue (EventDispatchers|CreateEvent :!event Custom|OnDeselectAllExcept))))

(fn FindItem
  (params (Item :type S%20Item%20Data%20Structure))
  (for _array_element (Variables|Default|Get_items)
    (bind _output_get (LocalVariables|SetCurrentSlot _array_element))
    (if (Variables|/Game/Blueprints/Systems/Inventory/BP_InventorySlot.BP_InventorySlot_C|GethasItem _output_get)
      (if (Utilities|Name|Equal(Name) (.name (Variables|/Game/Blueprints/Systems/Inventory/BP_InventorySlot.BP_InventorySlot_C|GetitemData (LocalVariables|GetCurrentSlot))) (.name Item))
        (return (LocalVariables|GetCurrentSlot) true))))
  (return 0 false))

(fn FindSlotforItem
  (params (Item :type S%20Item%20Data%20Structure))
  ;[1 1 1] Is the item stackable?
  (if (.Stackable (Utilities|Struct|BreakSItemData Item))
    ;[1 1 1] Find the stackable slot
    (bind (_slot _found_) (CallFunction|FindItem Item))
    (if _found_
      (return _slot true)
      (else
        _)))
  ;[1 1 1] Find first empty slot
  (for _array_element (Variables|Default|Get_items)
    (if (not (Variables|/Game/Blueprints/Systems/Inventory/BP_InventorySlot.BP_InventorySlot_C|GethasItem _array_element))
      (return _array_element true)))
  (return 0 false))

(fn SetSlot
  (params (Slot :type BP%20Inventory%20Slot%20Object%20Reference) (Item :type S%20Item%20Data%20Structure) (Quantity :type Integer))
  ;[1 1 1] Add a new item
  (Variables|/Game/Blueprints/Systems/Inventory/BP_InventorySlot.BP_InventorySlot_C|SetitemData Slot Item)
  (Variables|/Game/Blueprints/Systems/Inventory/BP_InventorySlot.BP_InventorySlot_C|SethasItem Slot true)
  ;[1 1 1] Add to the stackable item's current quantity
  (if (.Stackable (Utilities|Struct|BreakSItemData Item))
    (Variables|/Game/Blueprints/Systems/Inventory/BP_InventorySlot.BP_InventorySlot_C|Setquantity Slot (+ (Variables|/Game/Blueprints/Systems/Inventory/BP_InventorySlot.BP_InventorySlot_C|Getquantity Slot) Quantity))
    (Variables|/Game/Blueprints/Systems/Inventory/BP_InventorySlot.BP_InventorySlot_C|SethasItem Slot true)))

(fn GetIndex
  (params (Index :type Integer) (Columns :type Integer))
  (bind _returnvalue (+ Index 1))
  (return (/ _returnvalue Columns) (Math|Integer|%(Integer) _returnvalue Columns)))

(fn AddtoInventory
  (params (Item :type S%20Item%20Data%20Structure) (Quantity :type Integer))
  (bind (_slot _found_) (CallFunction|FindSlotforItem Item))
  (LocalVariables|SetSlot _slot)
  (if _found_
    (CallFunction|SetSlot (LocalVariables|GetSlot) Item Quantity)
    (Default|CallItemPickedUp (LocalVariables|GetSlot))
    (Default|CallChanged (LocalVariables|GetSlot))
    (Default|CallItemAdded)
    (return true)
    (else
      (Default|CallInventoryFull)
      (return false))))

(fn HasItem
  (params (Item :type S%20Item%20Data%20Structure))
  (for _array_element (Variables|Default|Get_items)
    (if true
      (return true)))
  (return false))