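; BP_CombatComponent is a combat component that loads its owner's combat info and gives that owner a nameplate actor.
; On BeginPlay, if its row handle's table is valid, it reads that row name from DT_CombatInfo, stores the result and spawns a BP_Nameplate at the owner's transform.
; Every Tick it teleports the nameplate to the owner's bounds BoxExtent, used directly as a world location without the bounds origin.
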(event EventBeginPlay
  (bind _returnvalue (Components|GetOwner))
  (bind _combatinforow (Variables|Default|GetCombatInfoRow))
  (Utilities|IsValid (.datatable _combatinforow)
    (:Is%20Valid
      (bind _returnvalue_2 (Utilities|GetDataTableRow "/Game/Blueprints/Systems/Combat/DT_CombatInfo.DT_CombatInfo" (.rowname _combatinforow))
        (:then
          (Variables|Default|SetCombatInfo _returnvalue_2)
          (bind _returnvalue_3 (Game|SpawnActorfromClass "/Game/Blueprints/Systems/Interaction/BP_Nameplate.BP_Nameplate_C" (Transformation|GetActorTransform _returnvalue) "AlwaysSpawn" _returnvalue 0))
          (Variables|Default|SetNameplate _returnvalue_3))))))

(event EventTick
  (params (DeltaSeconds :type Float%20%28single-precision%29))
  (CallFunction|UpdateNameplatePosition))

(fn UpdateNameplatePosition
  (Transformation|SetActorLocation (Variables|Default|GetNameplate) (.BoxExtent (Collision|GetActorBounds (Components|GetOwner) false false)) false true))