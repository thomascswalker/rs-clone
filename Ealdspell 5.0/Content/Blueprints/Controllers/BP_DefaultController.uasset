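; Player controller for a point-and-click game that drives the player character's camera, creates the HUD and toggles the inventory.
; Axis inputs change camera FOV and rotate the spring arm within zoom and pitch limits.
; Left click traces under the cursor, clears the character's TaskComponent queue and queues a BPT_Move task.
; For IInteractive targets, it also queues the first task from that actor's interactive component, chaining move then action.
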(event EventBeginPlay
  ;[1 1 1] Possess the camera
  (Game|Player|SetViewTargetwithBlend (Variables|Default|GetPlayerCharacter) 0.0 "VTBlend_Linear" 0.0 false)
  ;[1 1 1] Initialize the user interface
  (CallFunction|InitializeInterface))

(event Input|AxisEvents|InputAxisCameraUp
  (params (AxisValue :type Float%20%28single-precision%29))
  (bind _limit (Variables|Default|GetLimit))
  (bind _playercharacter (Variables|Default|GetPlayerCharacter))
  (bind _springarm (Variables|/Game/Blueprints/Controllers/BP_DefaultPlayerCharacter.BP_DefaultPlayerCharacter_C|GetSpringArm _playercharacter))
  (bind _returnvalue (Transformation|GetWorldRotation _springarm))
  ;[1 1 1] Camera up/down
  (Transformation|SetWorldRotation _springarm (Math|Rotator|MakeRotator (.roll _returnvalue) (Math|Float|Clamp(Float) (+ (* AxisValue (Variables|Default|GetCameraSpeed) (Utilities|Time|GetWorldDeltaSeconds)) (.pitch (Transformation|GetWorldRotation _springarm))) (.x _limit) (.y _limit)) (.yaw _returnvalue)) false false))

(event Input|AxisEvents|InputAxisCameraRight
  (params (AxisValue :type Float%20%28single-precision%29))
  ;[1 1 1] Camera left/right
  (Transformation|AddWorldRotation (Variables|/Game/Blueprints/Controllers/BP_DefaultPlayerCharacter.BP_DefaultPlayerCharacter_C|GetSpringArm (Variables|Default|GetPlayerCharacter)) (Math|Rotator|MakeRotator 0.0 0.0 (* AxisValue (Variables|Default|GetCameraSpeed) (Utilities|Time|GetWorldDeltaSeconds))) false false))

(event Input|AxisEvents|InputAxisCameraZoom
  (params (AxisValue :type Float%20%28single-precision%29))
  (bind _playercharacter (Variables|Default|GetPlayerCharacter))
  (bind _camera (Variables|/Game/Blueprints/Controllers/BP_DefaultPlayerCharacter.BP_DefaultPlayerCharacter_C|GetCamera _playercharacter))
  ;[1 1 1] Camera zoom
  (Camera|SetFieldOfView _camera (Math|Float|Clamp(Float) (+ (* AxisValue (Variables|Default|GetZoomSpeed) (Utilities|Time|GetWorldDeltaSeconds)) (Variables|/Script/Engine.CameraComponent|GetFieldOfView _camera)) 1e+01 9e+01)))

(event Input|MouseEvents|LeftMouseButton
  (params (Key :type Key%20Structure))
  ;[1 1 1] Left click
  (:Pressed
    (CallFunction|OnLeftClick)))

(event Input|KeyboardEvents|B
  (params (Key :type Key%20Structure))
  (bind _playercharacter (Variables|Default|GetPlayerCharacter))
  ;[1 1 1] Toggle inventory
  (:Released
    (Utilities|IsValid _playercharacter
      (:Is%20Valid
        (Default|Toggle (Variables|/Game/Blueprints/Controllers/BP_DefaultPlayerCharacter.BP_DefaultPlayerCharacter_C|GetInventoryComponent _playercharacter))))))

(fn ConstructionScript)

(fn OnLeftClick
  (bind (_hitresult _returnvalue) (Game|Player|GetHitResultUnderCursorbyChannel "TraceTypeQuery1" true))
  (bind _playercharacter (Variables|Default|GetPlayerCharacter))
  (bind _playercharacter_2 (Variables|Default|GetPlayerCharacter))
  (bind (_bblockinghit _binitialoverlap _time _distance _location _impactpoint _normal _impactnormal _physmat _hitactor) (Collision|BreakHitResult _hitresult))
  (bind _taskcomponent (Variables|/Game/Blueprints/Controllers/BP_DefaultPlayerCharacter.BP_DefaultPlayerCharacter_C|GetTaskComponent _playercharacter))
  (Utilities|FlowControl|Sequence
    (:then_0
      ;[1 1 1] Get what we hit
      (if _returnvalue
        (LocalVariables|SetLocation _location)
        (LocalVariables|SetHitActor _hitactor)
        (else
          (return))))
    (:then_1
      ;[1 1 1] Did we left click on an  object we can interact with?
      (bind _asiinteractive (Utilities|Casting|CastToIInteractive (LocalVariables|GetHitActor))
        (:then
          (bind _actor (Default|GetActor _asiinteractive))
          (Variables|Default|SetMoveAndAction true))
        (:CastFailed
          _))
      ;[1 1 1] Move to
      (bind _returnvalue_2 (Game|ConstructObjectfromClass (Variables|Default|GetPlayerCharacter) "/Game/Blueprints/Systems/Tasks/BPT_Move.BPT_Move_C" (LocalVariables|GetLocation) (LocalVariables|GetHitActor) (Variables|Default|GetMovementThreshold) _actor))
      (Default|ClearQueue _taskcomponent)
      (Default|OnAddTasktoQueue _taskcomponent _returnvalue_2)
      (if (Variables|Default|GetMoveAndAction)
        ;[1 1 1] Add the first task from the object we just clicked
        (bind _component (Class|IInteractive|GetInteractiveComponent(Message) _actor))
        (Utilities|IsValid _component
          (:Is%20Valid
            (bind _task (Default|GetTask _component))
            (if (Utilities|IsValidClass _task)
              (bind _returnvalue_3 (Game|ConstructObjectfromClass _playercharacter_2 _task _actor))
              (Default|OnAddTasktoQueue (Variables|/Game/Blueprints/Controllers/BP_DefaultPlayerCharacter.BP_DefaultPlayerCharacter_C|GetTaskComponent _playercharacter_2) _returnvalue_3))))))))

(fn InitializeInterface
  (bind _returnvalue (UserInterface|CreateWidget "/Game/Blueprints/Systems/Interface/WBP_HUD.WBP_HUD_C" self))
  (UserInterface|Viewport|AddtoViewport _returnvalue -999))