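; Default player character that projects a decal at the world point under the mouse cursor, aligned to the surface normal every tick.
; SpawnItem traces down from the character and spawns a BP_Item from the item data table at the hit location.
; Getter functions expose the controller, HUD, combat and task components, though several return nothing.
; Task progress bar functions are unfinished, with viewport add and removal left unconnected.
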(event EventTick
  (params (DeltaSeconds :type Float%20%28single-precision%29))
  (bind _returnvalue (Game|GetPlayerController 0))
  (bind _hitresult (Game|Player|GetHitResultUnderCursorbyChannel _returnvalue "TraceTypeQuery1" true))
  (bind (_bblockinghit _binitialoverlap _time _distance _location _impactpoint _normal _impactnormal) (Collision|BreakHitResult _hitresult))
  (Transformation|SetWorldLocationAndRotation (Variables|Default|GetDecal) _location (Math|Rotator|MakeRotationfromAxes _impactnormal "0, 0, 0" "0, 0, 0") false false))

(fn ConstructionScript)

(fn SpawnItem
  (params (Item :type S%20Item%20Data%20Structure) (Quantity :type Integer))
  (bind _returnvalue (Transformation|GetActorTransform))
  (bind (_x _y) (Math|Vector|BreakVector (.location _returnvalue)))
  (bind _outhit (Collision|LineTraceByChannel (.location _returnvalue) (Math|Vector|MakeVector _x _y -1e+04) "TraceTypeQuery1" false 0 "None"))
  (bind _returnvalue_2 (Game|SpawnActorfromClass "/Game/Blueprints/Systems/Items/BP_Item.BP_Item_C" (Math|Transform|MakeTransform (.Location (Collision|BreakHitResult _outhit)) "0, 0, 0" "1.000000,1.000000,1.000000") "AdjustIfPossibleButAlwaysSpawn" 0 (Utilities|Struct|MakeDataTableRowHandle "/Game/Blueprints/Systems/Items/DT_ItemTable.DT_ItemTable" (.Name (Utilities|Struct|BreakSItemData Item))) Quantity 0))
  (return (Utilities|IsValid _returnvalue_2)))

(fn ConstructProgressBar
  (params (Task :type BP%20Task%20Object%20Reference))
  (UserInterface|CreateWidget "/Game/Blueprints/Systems/Tasks/WBP_TaskProgress.WBP_TaskProgress_C" 0 (Variables|/Game/Blueprints/Systems/Tasks/BP_Task.BP_Task_C|GetProgressMessage Task) (Variables|/Game/Blueprints/Systems/Tasks/BP_Task.BP_Task_C|GetProgressTime Task)))

(fn DestroyProgressBar
  (Utilities|IsValid 0))

(fn GetPlayerController
  (bind _asbp_default_controller (Utilities|Casting|CastToBP_DefaultController (Game|GetPlayerController 0)))
  (return _asbp_default_controller))

(fn GetActor
  (return 0))

(fn GetAiController
  (return (AI|GetAIController self)))

(fn GetCharacter
  (return self))

(fn GetCombatComponent
  (return (Variables|Default|GetCombatComponent)))

(fn GetDisplayName
  (return ""))

(fn GetHighlightableMesh
  (return 0))

(fn GetHud
  (bind _foundwidgets (Widget|GetAllWidgetsOfClass "/Game/Blueprints/Systems/Interface/WBP_HUD.WBP_HUD_C" false))
  (for _array_element _foundwidgets
    (return _array_element)))

(fn GetInteractiveComponent
  (return 0))

(fn GetProgressBar
  (return 0))

(fn GetSkillComponent
  (return 0))

(fn GetTaskComponent
  (return (Variables|Default|GetTaskComponent)))

(fn GetWidget
  (params (Widget :type User%20Widget%20Class%20Reference))
  (bind _foundwidgets (Widget|GetAllWidgetsOfClass Widget true))
  (for _array_element _foundwidgets
    (return _array_element)))