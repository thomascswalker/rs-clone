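; Interaction component that makes its IInteractive owner highlightable under the cursor and shows a hover prompt on the player's HUD.
; On BeginPlay it binds cursor events on the owner's highlightable mesh and adds a colored outline material to a camera's post-process settings.
; Hovering toggles the mesh's custom depth for the outline and shows or hides rich text combining the first task's name with the owner's display name.
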(event Custom|OnHover
  (params (TouchedObject :type Primitive%20Component%20Object%20Reference))
  (CallFunction|UpdateHoverText true TouchedObject))

(event Custom|OnDehover
  (params (TouchedObject :type Primitive%20Component%20Object%20Reference))
  (CallFunction|UpdateHoverText false TouchedObject))

(event EventBeginPlay
  (CallFunction|Initialize))

(fn GetTask
  (params (Index :type Integer))
  (return (Utilities|Array|Get(acopy) (Variables|Default|GetTasks) Index)))

(fn UpdateHoverText
  (params (hovered :type Boolean) (object :type Primitive%20Component%20Object%20Reference))
  (Rendering|SetRenderCustomDepth object hovered)
  (bind _asbp_default_controller (Utilities|Casting|CastToBP_DefaultController (Game|GetPlayerController 0)))
  (bind _hud (Class|BPITaskExecutor|GetHud(Message) (Variables|/Game/Blueprints/Controllers/BP_DefaultController.BP_DefaultController_C|GetPlayerCharacter _asbp_default_controller)))
  (if hovered
    (Default|ShowHoverText _hud (CallFunction|GetHoverText))
    (else
      (Default|HideHoverText _hud))))

(fn GetHoverText
  ;[1 1 1] Object name
  (bind _asiinteractive (Utilities|Casting|CastToIInteractive (Components|GetOwner)))
  (bind _displayname (Default|GetDisplayName _asiinteractive))
  (return (Utilities|String|JoinStringArray (Utilities|Array|MakeArray (.DisplayName (Utilities|GetClassDefaults (Utilities|Array|Get(acopy) (Variables|Default|GetTasks)))) "<Item>" _displayname "</>") " ")))

(fn Initialize
  (if (Utilities|DoesObjectImplementInterface (Components|GetOwner) "/Game/Blueprints/Systems/Interaction/IInteractive.IInteractive_C")
    (bind _asiinteractive (Utilities|Casting|CastToIInteractive (Components|GetOwner)))
    (bind _mesh (Default|GetHighlightableMesh _asiinteractive))
    (EventDispatchers|BindEventtoOnBeginCursorOver _mesh (EventDispatchers|CreateEvent :!event Custom|OnHover))
    (EventDispatchers|BindEventtoOnEndCursorOver _mesh (EventDispatchers|CreateEvent :!event Custom|OnDehover))
    (Rendering|SetRenderCustomDepth _mesh false)
    (Rendering|SetCustomDepthStencilValue _mesh 1)
    (bind _returnvalue (Rendering|Material|CreateDynamicMaterialInstance "/Game/Materials/M_OutlineInstance.M_OutlineInstance" "None" "None" :!class /Script/Engine.KismetMaterialLibrary))
    (Rendering|Material|SetVectorParameterValue _returnvalue "Color" "(R=1.000000,G=0.004504,B=0.000000,A=1.000000)" :!class /Script/Engine.MaterialInstanceDynamic)
    (bind _output_get (Variables|Default|SetOutlineMaterial _returnvalue))
    (Utilities|Struct|SetmembersinPostProcessSettings (Variables|/Script/Engine.CameraComponent|GetPostProcessSettings (Actor|GetComponentbyClass "/Script/Engine.CameraComponent")) (Utilities|Struct|MakeWeightedBlendables (Utilities|Array|MakeArray (Utilities|Struct|MakeWeightedBlendable 1.0 _output_get))))))