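; BP_Skill is a single skill that tracks its own experience and level.
; AddExperience adds to the running total, broadcasts the gain, then raises Level at most once per call and broadcasts the level-up.
; The CanLevelUp macro passes when Experience exceeds the current level's threshold, queried from the owning BP_SkillComponent, found by casting the skill's Outer object.
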(fn AddExperience
  (params (ExperienceGained :type Integer))
  (bind _output_get (Variables|Default|SetExperience (+ ExperienceGained (Variables|Default|GetExperience))))
  (Default|CallGainedExperience ExperienceGained _output_get)
  (Utilities|CanLevelUp?
    (:Yes
      (bind _result (Math|Integer|IncrementInt (Variables|Default|GetLevel))
        (:%20%20
          (Default|CallLeveledUp _result))))))

(fn GetSkillComponent
  (bind _asskill_component (Utilities|Casting|CastToBP_SkillComponent (Utilities|GetOuterObject self)))
  (return _asskill_component))